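; Quest component that runs the quest-giver conversation and manages the dialog, quest-selection and quest HUD widgets.
; Each Quest call for a giver without an accepted quest advances the Dialog array, then opens the quest widget filled from Quests, or closes it if already active.
; Opening dialog enables cursor and UI input; closing the quest widget restores game-only input.
; A HUD, created hidden on BeginPlay, shows the active quest's title and objectives.
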(event Custom|Close%20Widget
  (bind _returnvalue (Game|GetPlayerController 0))
  ;[0.15 0.15 0.15 0.5] Close Quest Widget
  (Widget|RemovefromParent (Variables|Default|GetQuest%20Widget))
  (Variables|Default|SetQuest%20Widget 0)
  (Variables|/Script/Engine.PlayerController|SetbShowMouseCursor _returnvalue false)
  (Input|SetInputModeGameOnly _returnvalue false)
  (Variables|Default|SetWidget%20Active false))

(event Custom|Open%20Quest%20Widget
  ;[0.15 0.15 0.15 0.5] Open Quest Widget
  (bind _ownerquestgiver (Variables|Default|GetOwnerQuestGiver)
    (:then
      (bind _returnvalue (UserInterface|CreateWidget "/Game/Arbin/Blueprints/QuestSystem/WBP_QuestGiver.WBP_QuestGiver_C"))
      (bind _output_get (Variables|Default|SetQuest%20Widget _returnvalue))
      (UserInterface|Viewport|AddtoViewport _output_get 0)
      (Variables|Default|SetWidget%20Active true)
      (Variables|/Game/Arbin/Blueprints/QuestSystem/WBP_QuestGiver.WBP_QuestGiver_C|SetQuest%20Giver (Variables|Default|GetQuest%20Widget) _ownerquestgiver)
      (for _array_element (Variables|Default|GetQuests)
        (Default|AddQuest (Variables|Default|GetQuest%20Widget) _array_element)))
    (:else
      (Development|PrintString "Hello" true true "(R=1.000000,G=0.425352,B=0.000000,A=1.000000)"))))

(event Custom|Set%20Active%20Quest%20Text
  (bind _quest_hud_widget (Variables|Default|GetQuest%20HUD%20Widget))
  ;[0.15 0.15 0.15 0.5] Fill Quest HUD
  (Rendering|Components|TextRender|SetText (Variables|/Game/Arbin/Blueprints/QuestSystem/WBP_QuestHUD.WBP_QuestHUD_C|GetActiveTextQuest _quest_hud_widget) (Utilities|Text|ToText(String) (.Title (Utilities|Struct|BreakS_Quest (Variables|Default|GetActive%20Quest)))))
  (Widget|SetVisibility _quest_hud_widget "Visible"))

(event Custom|Set%20Objective
  ;[0.15 0.15 0.15 0.5] Fill Objectives
  (Default|FillObjectives (Variables|Default|GetQuest%20HUD%20Widget) (.objectives (Variables|Default|GetActive%20Quest))))

(event Custom|Quest
  (params (Owner :type BP%20AI%20Quest%20Giver%20Object%20Reference))
  (bind _returnvalue (Game|GetPlayerController 0))
  (Utilities|IsValid Owner
    (:Is%20Valid
      (if (not (Variables|/Game/Arbin/Blueprints/QuestSystem/BP_AI_QuestGiver.BP_AI_QuestGiver_C|GetbHasAcceptedQuest? Owner))
        (Variables|Default|SetOwnerQuestGiver Owner)
        (if (not (Variables|Default|GetWidget%20Active))
          ;[0.15 0.15 0.15 0.5] Next Quest Dialog
          (if (not (Variables|Default|GetDialogOpened?))
            ;[0.15 0.15 0.15 0.5] Open Quest Dialog Widget
            (bind _returnvalue_2 (UserInterface|CreateWidget "/Game/Arbin/Blueprints/QuestSystem/WBP_QuestGiver_dialog.WBP_QuestGiver_dialog_C"))
            (bind _output_get (Variables|Default|SetDialog%20Widget _returnvalue_2))
            (UserInterface|Viewport|AddtoViewport _output_get 0)
            (Variables|Default|SetDialogOpened? true)
            (Rendering|Components|TextRender|SetText (Variables|/Game/Arbin/Blueprints/QuestSystem/WBP_QuestGiver_dialog.WBP_QuestGiver_dialog_C|GetDialogText (Variables|Default|GetDialog%20Widget)) (Utilities|Text|ToText(String) (Utilities|Array|Get(acopy) (Variables|Default|GetDialog) (Variables|Default|GetDialog%20Index))))
            (Math|Integer|IncrementInt (Variables|Default|GetDialog%20Index)
              (:%20%20
                (Variables|/Script/Engine.PlayerController|SetbShowMouseCursor _returnvalue true)
                (Input|SetInputModeGameandUI _returnvalue (Variables|Default|GetQuest%20Widget) "DoNotLock" true false)))
            (else
              (Rendering|Components|TextRender|SetText (Variables|/Game/Arbin/Blueprints/QuestSystem/WBP_QuestGiver_dialog.WBP_QuestGiver_dialog_C|GetDialogText (Variables|Default|GetDialog%20Widget)) (Utilities|Text|ToText(String) (Utilities|Array|Get(acopy) (Variables|Default|GetDialog) (Variables|Default|GetDialog%20Index))))
              (Math|Integer|IncrementInt (Variables|Default|GetDialog%20Index)
                (:%20%20
                  (if (> (Variables|Default|GetDialog%20Index) (Utilities|Array|Length (Variables|Default|GetDialog)))
                    (Widget|RemovefromParent (Variables|Default|GetDialog%20Widget))
                    (Variables|Default|SetDialog%20Widget 0)
                    (Variables|Default|SetDialog%20Index 0)
                    (Variables|Default|SetDialogOpened? false)
                    (CallFunction|OpenQuestWidget))))))
          (else
            (CallFunction|CloseWidget)))))
    (:Is%20Not%20Valid
      (Development|PrintString "Hello" true true "(R=1.000000,G=0.425352,B=0.000000,A=1.000000)"))))

(event EventBeginPlay
  ;[0.15 0.15 0.15 0.5] Add Quest HUD
  (bind _returnvalue (UserInterface|CreateWidget "/Game/Arbin/Blueprints/QuestSystem/WBP_QuestHUD.WBP_QuestHUD_C"))
  (bind _output_get (Variables|Default|SetQuest%20HUD%20Widget _returnvalue))
  (UserInterface|Viewport|AddtoViewport _output_get 0)
  (Widget|SetVisibility _output_get "Hidden"))