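; Target lock-on component for BP_PastPlayer that locks the camera onto a nearby LockOnClass actor and can switch to targets on the left or right.
; Candidates come from a sphere trace, pass a line trace, and are ranked by dot product against camera forward; switching filters sides by hit normal versus camera right.
; While locked, a looping timer interpolates control rotation toward a distance-lowered aim point, character rotation follows the controller, and lock releases beyond LockOnRadius.
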(event Custom|Trigger%20Target%20Lock%20On
  (bind _targets (CallFunction|TraceforTargets))
  (bind _past_player (Variables|Default|GetPast%20Player))
  (bind _target_to_lock_on (CallFunction|CheckforClosestTarget _targets))
  (bind _charactermovement (Variables|/Script/Engine.Character|GetCharacterMovement _past_player))
  (Utilities|IsValid _target_to_lock_on
    (:Is%20Valid
      (Variables|Default|SetTargetLockOn _target_to_lock_on)
      (bind _output_get (Variables|Default|SetLockOn true))
      (Default|CallOnTargetLockonTriggered (Variables|Default|GetPast%20Player) _output_get)
      (Variables|/Script/Engine.CharacterMovementComponent|SetbOrientRotationToMovement _charactermovement false)
      (Variables|/Script/Engine.CharacterMovementComponent|SetbUseControllerDesiredRotation _charactermovement true)
      (Development|PrintString "tARGET lOCKED")
      (bind _returnvalue (Utilities|Time|SetTimerbyEvent (delegate Custom|Target%20Lock%20On) (Utilities|Time|GetWorldDeltaSeconds) true)))))

(event Custom|Target%20Lock%20On
  (bind _return (CallFunction|GetLockonCameraRotation))
  (bind _past_player (Variables|Default|GetPast%20Player))
  (bind _returnvalue (Pawn|GetController _past_player))
  (bind _returnvalue_2 (Pawn|GetControlRotation _returnvalue :!class /Script/Engine.Controller))
  (bind _returnvalue_3 (Math|Interpolation|RInterpTo _returnvalue_2 _return 0.01 1e+01))
  (bind _targetlockon (Variables|Default|GetTargetLockOn)
    (:then
      (if (> (Math|Vector|Distance(Vector) (Transformation|GetActorLocation (Variables|Default|GetPast%20Player)) (Transformation|GetActorLocation _targetlockon)) (Variables|Default|GetLockOnRadius))
        (CallFunction|StopTargetLockon)
        (Development|PrintString "Target Unlocked")
        (else
          (Pawn|SetControlRotation _returnvalue (Math|Rotator|MakeRotator (.Roll (Math|Rotator|BreakRotator _returnvalue_2)) (.pitch _returnvalue_3) (.yaw _returnvalue_3))))))
    (:else)))

(event Custom|Stop%20Target%20Lock%20On
  (bind _past_player (Variables|Default|GetPast%20Player))
  (bind _charactermovement (Variables|/Script/Engine.Character|GetCharacterMovement _past_player))
  (Utilities|Time|ClearandInvalidateTimerbyHandle (stale Custom|Trigger%20Target%20Lock%20On _returnvalue))
  (bind _output_get (Variables|Default|SetLockOn false))
  (Default|CallOnTargetLockonTriggered (Variables|Default|GetPast%20Player) _output_get)
  (Variables|/Script/Engine.CharacterMovementComponent|SetbOrientRotationToMovement _charactermovement true)
  (Variables|/Script/Engine.CharacterMovementComponent|SetbUseControllerDesiredRotation _charactermovement false))

(event Custom|Switch%20Target%20On%20Right
  (Utilities|IsValid (Variables|Default|GetTargetLockOn)
    (:Is%20Valid
      (bind _right_target (CallFunction|GetTargetonRight))
      (Utilities|IsValid _right_target
        (:Is%20Valid
          (Variables|Default|SetTargetLockOn _right_target))))))

(event Custom|Switch%20Target%20On%20Left
  (Utilities|IsValid (Variables|Default|GetTargetLockOn)
    (:Is%20Valid
      (bind _left_target (CallFunction|GetTargetonLeft))
      (Utilities|IsValid _left_target
        (:Is%20Valid
          (Variables|Default|SetTargetLockOn _left_target))))))

(event Custom|Foo
  (Development|PrintString "FOO"))

(event EventBeginPlay
  ;[0.15 0.15 0.15 0.5] Set Player
  (bind _asbp_past_player (Utilities|Casting|CastToBP_PastPlayer (Components|GetOwner)))
  (Variables|Default|SetPast%20Player _asbp_past_player))

(fn TraceforTargets
  (bind _past_player (Variables|Default|GetPast%20Player))
  (bind _returnvalue (Transformation|GetActorLocation _past_player))
  (bind (_outhits _returnvalue_2) (Collision|MultiSphereTraceForObjects _returnvalue _returnvalue (Variables|Default|GetLockOnRadius) (Utilities|Array|MakeArray "ObjectTypeQuery7") false 0 "None"))
  (if _returnvalue_2
    (for _array_element _outhits
      (if (Utilities|ClassIsChildOf (Utilities|GetClass (.HitActor (Collision|BreakHitResult _array_element))) (Variables|Default|GetLockOnClass))
        (Utilities|Array|Add (LocalVariables|GetLocalTargets) (.HitActor (Collision|BreakHitResult _array_element)))))
    (return (LocalVariables|GetLocalTargets))))

(fn CheckforClosestTarget
  (params (Targets :type Array%20of%20Actor%20Object%20References))
  (for _array_element Targets
    (bind _returnvalue (Collision|LineTraceByChannel (Transformation|GetWorldLocation (Variables|/Game/Arbin/Blueprints/BP_PastPlayer.BP_PastPlayer_C|GetFollowCamera (Variables|Default|GetPast%20Player))) (Transformation|GetActorLocation _array_element) "TraceTypeQuery1" false 0 "None"))
    (if _returnvalue
      (Math|Float|CompareFloat (CallFunction|CheckTargetCloseness _array_element) (LocalVariables|GetLocalCompareFloat)
        (:>
          (LocalVariables|SetLocalCompareFloat (CallFunction|CheckTargetCloseness _array_element))
          (LocalVariables|SetLocalTargetToLockOn _array_element)))))
  (return (LocalVariables|GetLocalTargetToLockOn)))

(fn CheckTargetCloseness
  (params (Target :type Actor%20Object%20Reference))
  (bind _past_player (Variables|Default|GetPast%20Player))
  (return (Math|Vector|DotProduct (Math|Vector|GetForwardVector (Variables|/Game/Arbin/Blueprints/BP_PastPlayer.BP_PastPlayer_C|GetFollowCamera _past_player)) (Math|Rotator|GetRotationXVector (Math|Rotator|FindLookatRotation (Transformation|GetActorLocation _past_player) (Transformation|GetActorLocation Target))))))

(fn GetLockonCameraRotation
  (bind _targetlockon (Variables|Default|GetTargetLockOn))
  (bind _returnvalue (Transformation|GetActorLocation _targetlockon))
  (return (Math|Rotator|FindLookatRotation (Transformation|GetWorldLocation (Variables|/Game/Arbin/Blueprints/BP_PastPlayer.BP_PastPlayer_C|GetFollowCamera (Variables|Default|GetPast%20Player))) (Math|Vector|MakeVector (.x _returnvalue) (.y _returnvalue) (- (.z _returnvalue) (/ (Math|Vector|Distance(Vector) (Transformation|GetActorLocation (Variables|Default|GetPast%20Player)) (Transformation|GetActorLocation (Variables|Default|GetTargetLockOn))) 2.0))))))

(fn GetTargetonLeft
  (for _array_element (CallFunction|TraceforTargets)
    (bind (_outhit _returnvalue) (Collision|LineTraceForObjects (Transformation|GetWorldLocation (Variables|/Game/Arbin/Blueprints/BP_PastPlayer.BP_PastPlayer_C|GetFollowCamera (Variables|Default|GetPast%20Player))) (Transformation|GetActorLocation _array_element) (Utilities|Array|MakeArray "ObjectTypeQuery7") false 0 "None"))
    (if _returnvalue
      (if (and (!= (Variables|Default|GetTargetLockOn) _array_element) (> (Class|KismetMathLibrary|DegAsin (Math|Vector|DotProduct (Math|Vector|GetRightVector (Variables|/Game/Arbin/Blueprints/BP_PastPlayer.BP_PastPlayer_C|GetFollowCamera (Variables|Default|GetPast%20Player))) (.Normal (Collision|BreakHitResult _outhit)))) 0.0))
        (Math|Float|CompareFloat (CallFunction|CheckTargetCloseness _array_element) (LocalVariables|GetLocalTargetCompare)
          (:>
            (LocalVariables|SetLocalTargetCompare (CallFunction|CheckTargetCloseness _array_element))
            (LocalVariables|SetLocalTargetToLock _array_element))))))
  (return (LocalVariables|GetLocalTargetToLock)))

(fn GetTargetonRight
  (for _array_element (CallFunction|TraceforTargets)
    (bind (_outhit _returnvalue) (Collision|LineTraceForObjects (Transformation|GetWorldLocation (Variables|/Game/Arbin/Blueprints/BP_PastPlayer.BP_PastPlayer_C|GetFollowCamera (Variables|Default|GetPast%20Player))) (Transformation|GetActorLocation _array_element) (Utilities|Array|MakeArray "ObjectTypeQuery7") false 0 "None"))
    (if _returnvalue
      (if (and (!= (Variables|Default|GetTargetLockOn) _array_element) (< (Class|KismetMathLibrary|DegAsin (Math|Vector|DotProduct (Math|Vector|GetRightVector (Variables|/Game/Arbin/Blueprints/BP_PastPlayer.BP_PastPlayer_C|GetFollowCamera (Variables|Default|GetPast%20Player))) (.Normal (Collision|BreakHitResult _outhit)))) 0.0))
        (Math|Float|CompareFloat (CallFunction|CheckTargetCloseness _array_element) (LocalVariables|GetLocalTargetCompare)
          (:>
            (LocalVariables|SetLocalTargetCompare (CallFunction|CheckTargetCloseness _array_element))
            (LocalVariables|SetLocalTargetToLock _array_element))))))
  (return (LocalVariables|GetLocalTargetToLock)))