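; Sword weapon Blueprint that the player picks up, equips and swings.
; Anim notify handlers snap it between equipped and unequipped character sockets and swap idle animations.
; Once picked up, it runs a four-hit light combo that buffers input and advances or resets on combo notifies, plus a random special montage gated by a delayed DoOnce cooldown.
; A Niagara effect shows while the player overlaps the trigger and is destroyed on pickup.
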(event OnComponentBeginOverlap(Trigger)
  (params (OverlappedComponent :type Primitive%20Component%20Object%20Reference) (OtherActor :type Actor%20Object%20Reference) (OtherComp :type Primitive%20Component%20Object%20Reference) (OtherBodyIndex :type Integer) (bFromSweep :type Boolean) (SweepResult :type Hit%20Result%20Structure%20%28by%20ref%29))
  ;[0.15 0.15 0.15 0.5] Niagara Efficet
  (if (Actor|ActorHasTag OtherActor "Player")
    (Components|Activation|Activate (Variables|Default|GetNiagara) false)))

(event OnComponentEndOverlap(Trigger)
  (params (OverlappedComponent :type Primitive%20Component%20Object%20Reference) (OtherActor :type Actor%20Object%20Reference) (OtherComp :type Primitive%20Component%20Object%20Reference) (OtherBodyIndex :type Integer))
  ;[0.15 0.15 0.15 0.5] Niagara Efficet
  (if (Actor|ActorHasTag OtherActor "Player")
    (bind _niagara (Variables|Default|GetNiagara)
      (:then
        (Components|Activation|Deactivate _niagara))
      (:else))))

(event Custom|Attack
  ;[1 1 1] Attack System
  ;;[1 1 1] Attack
  (if (Variables|Default|GetIsAttacking?)
    (Variables|Default|SetSaveAttack? true)
    (else
      (Variables|Default|SetIsAttacking? true)
      ;;[1 1 1] Attack Combo according to no of press
      (switch int (Variables|Default|GetAttackIndex)
        (:0
          (CallFunction|Attack1))
        (:1
          (CallFunction|Attack2))
        (:2
          (CallFunction|Attack3))
        (:3
          (CallFunction|Attack4))))))

(event Custom|Stop%20Attack
  ;[1 1 1] Attack System
  ;;[1 1 1] Stop Attack
  (Variables|Default|SetIsAttacking? false)
  (Variables|Default|SetAttackIndex 0))

(event Custom|Attack%201
  ;[1 1 1] Attack System
  ;;[1 1 1] Attack 1
  (Utilities|FlowControl|DoOnce false :!label _label
    (:Completed
      (Utilities|FlowControl|Delay 0.2)
      (Animation|Montage|PlayMontage (Variables|/Script/Engine.Character|GetMesh (Variables|Default|GetOwnerCharacter)) "/Game/Arbin/Combat/Animation/Player_CombatLight_Montage.Player_CombatLight_Montage"
        (:then
          (Variables|Default|SetAttackIndex 1)
          (goto _label Reset))))))

(event Custom|Attack%202
  ;[1 1 1] Attack System
  ;;[1 1 1] Attack 2
  (Utilities|FlowControl|DoOnce false :!label _label
    (:Completed
      (Utilities|FlowControl|Delay 0.2)
      (Animation|Montage|PlayMontage (Variables|/Script/Engine.Character|GetMesh (Variables|Default|GetOwnerCharacter)) "/Game/Arbin/Combat/Animation/Player_CombatLight2_Montage.Player_CombatLight2_Montage"
        (:then
          (Variables|Default|SetAttackIndex 2)
          (goto _label Reset))))))

(event Custom|Attack%203
  ;[1 1 1] Attack System
  ;;[1 1 1] Attack 3
  (Utilities|FlowControl|DoOnce false :!label _label
    (:Completed
      (Utilities|FlowControl|Delay 0.2)
      (Animation|Montage|PlayMontage (Variables|/Script/Engine.Character|GetMesh (Variables|Default|GetOwnerCharacter)) "/Game/Arbin/Combat/Animation/Player_CombatLight3_Montage.Player_CombatLight3_Montage"
        (:then
          (Variables|Default|SetAttackIndex 3)
          (goto _label Reset))))))

(event Custom|Attack%204
  ;[1 1 1] Attack System
  ;;[1 1 1] Attack 4
  (Utilities|FlowControl|DoOnce false :!label _label
    (:Completed
      (Utilities|FlowControl|Delay 0.2)
      (Animation|Montage|PlayMontage (Variables|/Script/Engine.Character|GetMesh (Variables|Default|GetOwnerCharacter)) "/Game/Arbin/Combat/Animation/Player_CombatLight4_Montage.Player_CombatLight4_Montage"
        (:then
          (Variables|Default|SetAttackIndex 4)
          (goto _label Reset))))))

(event EventSpecialAttack
  ;[1 1 1] Attack System
  ;;[1 1 1] Special Attack
  (bind _output_get (Variables|Default|SetCanAttack? (Variables|Default|GetHasBeenPickedUp)))
  (if _output_get
    (Utilities|FlowControl|DoOnce false :!label _label
      (:Completed
        (Animation|Montage|PlayMontage (Variables|/Script/Engine.Character|GetMesh (Variables|Default|GetOwnerCharacter)) (select (Math|Random|RandomBool) "/Game/Arbin/Combat/Animation/Player_Combat_Special2_Montage.Player_Combat_Special2_Montage" "/Game/Arbin/Combat/Animation/Player_Combat_Special1_Montage.Player_Combat_Special1_Montage")
          (:then
            (Utilities|FlowControl|Delay 7.0)
            (goto _label Reset)))))))

(event EventRecieveComboStopNotify
  ;[1 1 1] Attack System
  ;;[1 1 1] Stop Attack
  (Variables|Default|SetIsAttacking? false)
  (Variables|Default|SetAttackIndex 0))

(event EventForceUnequip
  ;[0.15 0.15 0.15 0.5] Equip & Unequip
  (Transformation|AttachComponentToComponent (Variables|/Script/Engine.Character|GetMesh (Variables|Default|GetOwnerCharacter)) (.unequipped (.SocketToAttachTo (Utilities|Struct|BreakS_WeaponAnimations (Variables|Default|GetWeaponMontages)))) "SnapToTarget" "SnapToTarget" "SnapToTarget" true))

(event EventInitiateAttack
  ;[1 1 1] Attack System
  ;;[1 1 1] Can Attack?
  (bind _output_get (Variables|Default|SetCanAttack? (Variables|Default|GetHasBeenPickedUp)))
  (if _output_get
    (CallFunction|Attack)))

(event EventRecieveComboNextNotify
  ;[1 1 1] Attack System
  ;;[1 1 1] Attack Combo
  (if (Variables|Default|GetSaveAttack?)
    (Variables|Default|SetSaveAttack? false)
    ;;[1 1 1] Attack Combo according to no of press
    (switch int (Variables|Default|GetAttackIndex)
      (:0
        (CallFunction|Attack1))
      (:1
        (CallFunction|Attack2))
      (:2
        (CallFunction|Attack3))
      (:3
        (CallFunction|Attack4)))
    (else
      (CallFunction|StopAttack))))

(event EventOnWeaponPickedUp
  (params (PickedBy :type BP%20Character%20Base%20Object%20Reference))
  ;[0.15 0.15 0.15 0.5] Niagara Efficet
  (|CallParentFunction PickedBy)
  (Components|DestroyComponent (Variables|Default|GetNiagara)))

(event EventHandleEquipNotify
  ;[0.15 0.15 0.15 0.5] Equip & Unequip
  (CallFunction|ForceEquip)
  (Default|ChangeIdleAnimation (Variables|Default|GetOwnerCharacter) (Utilities|Array|Get(acopy) (.idle (Variables|Default|GetWeaponMontages))))
  (Variables|Default|SetEquipState "NewEnumerator2"))

(event EventHandleUnequipNotify
  ;[0.15 0.15 0.15 0.5] Equip & Unequip
  (CallFunction|ForceUnequip)
  (Default|ChangeIdleAnimation (Variables|Default|GetOwnerCharacter))
  (Variables|Default|SetEquipState "NewEnumerator4"))

(event EventForceEquip
  ;[0.15 0.15 0.15 0.5] Equip & Unequip
  (Transformation|AttachComponentToComponent (Variables|/Script/Engine.Character|GetMesh (Variables|Default|GetOwnerCharacter)) (.equipped (.SocketToAttachTo (Utilities|Struct|BreakS_WeaponAnimations (Variables|Default|GetWeaponMontages)))) "SnapToTarget" "SnapToTarget" "SnapToTarget" true))

(fn ConstructionScript)

(fn GetMeleeWeapon
  (return 0))