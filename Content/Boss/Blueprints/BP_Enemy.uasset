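; Boss enemy Blueprint that plays the montages for its attack, ability, roar and ultimate actions.
; Each Handle event plays its montage on the Mesh at a variable play rate.
; Both completion and interruption call that action's matching OnEnd dispatcher, so an interrupted montage still signals that the action has ended.
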(event Custom|HandleAbility1
  (Animation|Montage|PlayMontage (Variables|Character|GetMesh) (Variables|Default|GetAbility1Montage) (Variables|Default|GetAbility1Rate)
    (:OnCompleted
      _)
    (:OnInterrupted
      _))
  (Default|CallOnAbility1End))

(event Custom|HandleUltimate
  (Animation|Montage|PlayMontage (Variables|Character|GetMesh) (Variables|Default|GetUltimateMontage) (Variables|Default|GetUltimateRate)
    (:OnCompleted
      _)
    (:OnInterrupted
      _))
  (Default|CallOnUltimateEnd))

(event Custom|HandleAttack
  (Animation|Montage|PlayMontage (Variables|Character|GetMesh) (Variables|Default|GetAttackMontage) (Variables|Default|GetAttackPlayRate)
    (:OnCompleted
      _)
    (:OnInterrupted
      _))
  (Default|CallOnAttackEnd))

(event Custom|HandleRoar
  (Animation|Montage|PlayMontage (Variables|Character|GetMesh) (Variables|Default|GetRoarMontage) (Variables|Default|GetRoarRate)
    (:OnCompleted
      _)
    (:OnInterrupted
      _))
  (Default|CallOnRoarEnd))

(fn ConstructionScript)