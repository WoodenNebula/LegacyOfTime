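; Health component for BP_CharacterBase characters, handling damage, healing, stun, death and respawn, plus player-only health bar, low-health alert and camera shake.
; Damage is gated by death state and i-frames, then restarts a cooldown for ticking passive heal; timers also drive damage over time, stun and respawn invulnerability.
; Health and death-state dispatchers broadcast changes, with death running through montage-driven stages.
; Includes K/H debug keys and unused ragdoll events.
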(event Custom|FinishDeath
  ;[0.15 0.15 0.15 0.5] Death Finish
  (Utilities|FlowControl|Sequence
    (:then_0
      (Default|ChangeIdleAnimation (Variables|Default|GetOwnerCharacter) (Variables|Animations|GetDeathLoop)))
    (:then_1
      (bind _output_get (Variables|Health|SetDeathState "NewEnumerator2"))
      (Default|CallOnDeathStateChanged _output_get))))

(event Custom|StartDeath
  (bind _ownercharacter (Variables|Default|GetOwnerCharacter))
  ;[0.15 0.15 0.15 0.5] Death Start
  (Utilities|FlowControl|Sequence
    (:then_0
      (Pawn|Components|CharacterMovement|DisableMovement (Variables|/Script/Engine.Character|GetCharacterMovement _ownercharacter))
      (Collision|SetCollisionEnabled (Variables|/Script/Engine.Character|GetCapsuleComponent _ownercharacter) "NoCollision"))
    (:then_1
      (CallFunction|ClearAllTimers))
    (:then_2
      (bind _deathanimation (Variables|Animations|GetDeathAnimation)
        (:then
          (Animation|Montage|PlayMontage (Variables|/Script/Engine.Character|GetMesh (Variables|Default|GetOwnerCharacter)) _deathanimation
            (:OnCompleted
              _)
            (:OnInterrupted
              _)))
        (:else
          _))
      (CallFunction|FinishDeath))
    (:then_3
      (bind _output_get (Variables|Health|SetDeathState "NewEnumerator1"))
      (Default|CallOnDeathStateChanged _output_get))))

(event Custom|StartPassiveHeal
  ;[0.15 0.15 0.15 0.5] Passive Heal
  (Development|PrintString "Passive Healing Started")
  (bind _returnvalue (Utilities|Time|SetTimerbyEvent (delegate Custom|TimelyHeal) (Variables|PassiveHealing|GetPassiveHealTickRate) true true))
  (Variables|PassiveHealing|SetPassiveHealTickerTimer _returnvalue))

(event Custom|TimelyHeal
  ;[0.15 0.15 0.15 0.5] Passive Heal
  (CallFunction|Heal 5)
  (if (== (Variables|Health|GetHealth) (Variables|Health|GetMaxHealth))
    (Development|PrintString "Invalidating Passive heal Since Max Health")
    (Utilities|Time|ClearandInvalidateTimerbyHandle (Variables|PassiveHealing|GetPassiveHealTickerTimer))))

(event Custom|Init
  ;[0.15 0.15 0.15 0.5] Set Character Reference
  (bind _asbp_character_base (Utilities|Casting|CastToBP_CharacterBase (Components|GetOwner)))
  (Variables|Default|SetOwnerCharacter _asbp_character_base)
  (Utilities|FlowControl|Sequence
    (:then_0
      (if (Default|IsPlayerCharacter? (Variables|Default|GetOwnerCharacter))
        (CallFunction|CreatePlayerHealthWidget)))
    (:then_1
      (CallFunction|ResetPassiveHealTimer))
    (:then_2
      (EventDispatchers|AssignOnHealthChanged (EventDispatchers|CreateEvent :!event Custom|CheckDeath)))))

(event Custom|Heal
  (params (HealAmount :type Integer))
  ;[0.15 0.15 0.15 0.5] Heal
  (bind _output_get (Variables|Health|SetHealth (Math|Integer|Min(Integer) (+ (Variables|Health|GetHealth) HealAmount) (Variables|Health|GetMaxHealth))))
  (Default|CallOnHealthChanged _output_get false))

(event Custom|CheckDeath
  (params (NewHealth :type Integer) (WasDamaged? :type Boolean))
  ;[0.15 0.15 0.15 0.5] Check if character is dead
  (if (<= NewHealth 0)
    (CallFunction|StartDeath)
    (bind _damagealert (Variables|Default|GetDamageAlert)
      (:then
        (Widget|SetVisibility _damagealert "Hidden"))
      (:else))
    (elif (Actor|ActorHasTag (Variables|Default|GetOwnerCharacter) "Player")
      (if (< (CallFunction|GetNormalizedHealth) 0.21)
        (Variables|Default|GetDamageAlert
          (:then
            _)
          (:else
            (bind _returnvalue (UserInterface|CreateWidget "/Game/Commons/Widgets/WBP_DamageAlert.WBP_DamageAlert_C"))
            (bind _output_get (Variables|Default|SetDamageAlert _returnvalue))))
        (UserInterface|Viewport|AddtoViewport _output_get 0)
        (Widget|SetVisibility _output_get "Visible")
        (else
          (bind _damagealert_2 (Variables|Default|GetDamageAlert)
            (:then
              (Widget|SetVisibility _damagealert_2 "Hidden"))
            (:else)))))))

(event Custom|Respawn
  ;[0.15 0.15 0.15 0.5] Respawn
  (CallFunction|Heal (Variables|Health|GetMaxHealth))
  (Variables|Health|SetDeathState "NewEnumerator0")
  (Variables|Damage|SetIFrameActive true)
  (Utilities|Time|SetTimerbyEvent (delegate Custom|DisableIFrame) (Variables|Damage|GetIFrameTime)))

(event Custom|DisableIFrame
  ;[0.15 0.15 0.15 0.5] Respawn
  (Variables|Damage|SetIFrameActive false))

(event Custom|EndRagdoll
  (bind _ownercharacter (Variables|Default|GetOwnerCharacter))
  (bind _mesh (Variables|/Script/Engine.Character|GetMesh _ownercharacter))
  ;[0.15 0.15 0.15 0.5] Unused
  (Physics|SetSimulatePhysics _mesh false)
  (Collision|SetCollisionProfileName _mesh "CharacterMesh" false :!class /Script/Engine.PrimitiveComponent)
  (Transformation|AttachComponentToComponent _mesh (Variables|/Script/Engine.Character|GetCapsuleComponent (Variables|Default|GetOwnerCharacter)) "" "SnapToTarget" "SnapToTarget" "SnapToTarget" true))

(event Custom|StartRagdoll
  (bind _ownercharacter (Variables|Default|GetOwnerCharacter))
  (bind _mesh (Variables|/Script/Engine.Character|GetMesh _ownercharacter))
  ;[0.15 0.15 0.15 0.5] Unused
  (Collision|SetCollisionProfileName _mesh "Ragdoll" false :!class /Script/Engine.PrimitiveComponent)
  (Physics|SetSimulatePhysics _mesh true))

(event Input|KeyboardEvents|K
  (params (Key :type Key%20Structure :default "None"))
  (:Pressed
    (if (Default|IsPlayerCharacter? (Variables|Default|GetOwnerCharacter))
      (Development|PrintString "Self Destructing")
      (Variables|Damage|SetIFrameActive false)
      (CallFunction|DamageOverTime 4.0 25))))

(event Input|KeyboardEvents|H
  (params (Key :type Key%20Structure :default "None"))
  (:Pressed
    (if (Default|IsPlayerCharacter? (Variables|Default|GetOwnerCharacter))
      (Development|PrintString "Healing")
      (CallFunction|Respawn))))

(event Custom|ResetStun
  ;[0.15 0.15 0.15 0.5] Stun logic
  (Variables|Damage|SetbIsStunned? false)
  (Animation|StopAnimMontage (Variables|Default|GetOwnerCharacter) (Variables|Animations|GetStunLoop)))

(event Custom|PlayDamagedEffect
  (params (CameraShakeScale :type Float%20%28double-precision%29))
  ;[0.15 0.15 0.15 0.5] DamageEffect
  (if (Default|IsPlayerCharacter? (Variables|Default|GetOwnerCharacter))
    (Class|LegacyCameraShake|StartLegacyCameraShake (Variables|/Script/Engine.PlayerController|GetPlayerCameraManager (Pawn|GetLocalViewingPlayerController (Variables|Default|GetOwnerCharacter))) "/Game/Commons/Weapons/Ranged/BP_CameraShake.BP_CameraShake_C" CameraShakeScale "CameraLocal" "1.000000,1.000000,1.000000")))

(event Custom|DamageOverTime
  (params (Time :type Float%20%28double-precision%29) (DamagePerTick :type Integer))
  ;[0.15 0.15 0.15 0.5] Damage Over Time
  (Utilities|Time|SetTimerbyEvent (delegate Custom|Reset%20Timer) Time)
  (bind _returnvalue (Utilities|Time|SetTimerbyEvent (delegate Custom|ApplyTimelyDamage) (Variables|Damage|GetDamageTickRate) true true))
  (Variables|Damage|SetDamageOverTimeTimer _returnvalue))

(event Custom|ApplyTimelyDamage
  ;[0.15 0.15 0.15 0.5] Damage Over Time
  (CallFunction|Damage (stale Custom|DamageOverTime DamagePerTick) false 0.0))

(event Custom|Reset%20Timer
  ;[0.15 0.15 0.15 0.5] Damage Over Time
  (Utilities|Time|ClearandInvalidateTimerbyHandle (Variables|Damage|GetDamageOverTimeTimer)))

(event Custom|SelfDestruct
  ;[0.15 0.15 0.15 0.5] SelfDestruct
  (CallFunction|Damage (Variables|Health|GetHealth) false 0.0))

(event Custom|Damage
  (params (DamageAmount :type Integer) (Stun :type Boolean) (StunTime :type Float%20%28double-precision%29))
  ;[0.15 0.15 0.15 0.5] Apply Damage
  (if (CallFunction|CanTakeDamage)
    (Variables|Health|SetHealth (Math|Integer|Max(Integer) (- (Variables|Health|GetHealth) DamageAmount)))
    (CallFunction|ResetPassiveHealTimer)
    (CallFunction|PlayDamagedEffect (+ (/ (Math|Conversions|ToFloat(Integer) DamageAmount) (Math|Conversions|ToFloat(Integer) (Variables|Health|GetMaxHealth))) 0.4))
    (Default|CallOnHealthChanged (Variables|Health|GetHealth) true)
    (else
      (|DamageBlockReason:_2))))

(event Custom|Stun
  (params (StunTime :type Float%20%28double-precision%29))
  ;[0.15 0.15 0.15 0.5] Stun logic
  (Variables|Damage|SetbIsStunned? true)
  (Utilities|Time|SetTimerbyEvent (delegate Custom|ResetStun) StunTime)
  (Pawn|Components|CharacterMovement|DisableMovement (Variables|/Script/Engine.Character|GetCharacterMovement (Variables|Default|GetOwnerCharacter)))
  (Animation|Montage|PlayMontage (Variables|/Script/Engine.Character|GetMesh (Variables|Default|GetOwnerCharacter)) (Variables|Animations|GetStunStart)
    (:OnCompleted
      _)
    (:OnInterrupted
      _))
  (Animation|Montage|PlayMontage (Variables|/Script/Engine.Character|GetMesh (Variables|Default|GetOwnerCharacter)) (Variables|Animations|GetStunLoop)))

(fn CanHeal
  (return (and (< (CallFunction|GetNormalizedHealth) 1.0) (Utilities|Enum|Equal(Enum) (Variables|Health|GetDeathState) "NewEnumerator0"))))

(fn CanTakeDamage
  (return (Math|Boolean|ANDBoolean (> (CallFunction|GetNormalizedHealth) 0.0) (Utilities|Enum|Equal(Enum) (Variables|Health|GetDeathState) "NewEnumerator0") (not (Variables|Damage|GetIFrameActive)))))

(fn GetNormalizedHealth
  (return (Math|Float|SafeDivide (Math|Conversions|ToFloat(Integer) (Variables|Health|GetHealth)) (Math|Conversions|ToFloat(Integer) (Variables|Health|GetMaxHealth)))))

(fn ResetPassiveHealTimer
  (Development|PrintString "Reset Passive heal timer")
  (bind _returnvalue (Utilities|Time|SetTimerbyEvent (EventDispatchers|CreateEvent :!event Custom|StartPassiveHeal) (Variables|PassiveHealing|GetPassiveHealCooldownTime)))
  (Variables|PassiveHealing|SetPassiveHealStartTimer _returnvalue)
  (Utilities|Time|ClearandInvalidateTimerbyHandle (Variables|PassiveHealing|GetPassiveHealTickerTimer)))

(fn ClearAllTimers
  (Utilities|Time|ClearandInvalidateTimerbyHandle (Variables|Damage|GetDamageOverTimeTimer))
  (Utilities|Time|ClearandInvalidateTimerbyHandle (Variables|PassiveHealing|GetPassiveHealStartTimer))
  (Utilities|Time|ClearandInvalidateTimerbyHandle (Variables|PassiveHealing|GetPassiveHealTickerTimer)))

(fn CreatePlayerHealthWidget
  (Variables|Widgets|GetW_Healthbar
    (:then
      _)
    (:else
      (bind _returnvalue (UserInterface|CreateWidget "/Game/Commons/Widgets/WBP_Healthbar.WBP_Healthbar_C"))
      (bind _output_get (Variables|Widgets|SetW_Healthbar _returnvalue))
      (UserInterface|Viewport|AddtoViewport _output_get 0)))
  (Default|Init (Variables|Widgets|GetW_Healthbar) self))

(fn CreatePlayerDeathWidget)