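; Common game mode that saves, loads and clears the game through a single BP_SaveGame slot, loading automatically on BeginPlay.
; SaveGame stores the player's location, character reference and primary and secondary weapons, then sets the GameSlot flag, which NewGame clears when deleting the slot.
; LoadPlayerParameter teleports the player to the saved location but copies current weapons into the save object rather than restoring them.
; Disconnected older save and load nodes remain.
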(event Custom|New%20Game
  (SaveGame|DeleteGameinSlot (Variables|Default|GetSaveGameSlot))
  (Variables|Default|SetGameSlot? false))

(event Custom|Load%20Game
  ;[0.15 0.15 0.15 0.5] Load Game
  (bind _returnvalue (SaveGame|DoesSaveGameExist (Variables|Default|GetSaveGameSlot)))
  (if _returnvalue
    (bind _returnvalue_2 (SaveGame|LoadGamefromSlot (Variables|Default|GetSaveGameSlot)))
    (bind _asbp_save_game (Utilities|Casting|CastToBP_SaveGame _returnvalue_2))
    (Variables|Default|SetSaveGameBP _asbp_save_game)
    (CallFunction|LoadPlayerParameter)
    (Development|PrintString "Game Loaded")
    (else
      (Development|PrintString "Save Game First"))))

(event Custom|Save%20Game
  ;[0.15 0.15 0.15 0.5] Save Game
  (bind _returnvalue (SaveGame|DoesSaveGameExist (Variables|Default|GetSaveGameSlot)))
  (if _returnvalue
    _
    (else
      (bind _returnvalue_2 (SaveGame|CreateSaveGameObject "/Game/Commons/SaveLoad/BP_SaveGame.BP_SaveGame_C"))
      (Variables|Default|SetSaveGameBP _returnvalue_2)))
  (bind _asbp_player_character_base (Utilities|Casting|CastToBP_PlayerCharacterBase (Game|GetPlayerCharacter 0)))
  (Variables|/Game/Commons/SaveLoad/BP_SaveGame.BP_SaveGame_C|SetPlayerLocation (Variables|Default|GetSaveGameBP) (Transformation|GetActorLocation _asbp_player_character_base))
  (Variables|/Game/Commons/SaveLoad/BP_SaveGame.BP_SaveGame_C|SetPrimary%20Weapon (Variables|Default|GetSaveGameBP) (Variables|/Game/Commons/Weapons/Blueprints/BPC_WeaponInventoryComponent.BPC_WeaponInventoryComponent_C|GetPrimaryWeapon (Variables|/Game/Commons/Character/BP_CharacterBase.BP_CharacterBase_C|GetWeaponInventory _asbp_player_character_base)))
  (Variables|/Game/Commons/SaveLoad/BP_SaveGame.BP_SaveGame_C|SetSecondary%20Weapon (Variables|Default|GetSaveGameBP) (Variables|/Game/Commons/Weapons/Blueprints/BPC_WeaponInventoryComponent.BPC_WeaponInventoryComponent_C|GetSecondaryWeapon (Variables|/Game/Commons/Character/BP_CharacterBase.BP_CharacterBase_C|GetWeaponInventory _asbp_player_character_base)))
  (Variables|/Game/Commons/SaveLoad/BP_SaveGame.BP_SaveGame_C|SetPlayer (Variables|Default|GetSaveGameBP) _asbp_player_character_base)
  (SaveGame|SaveGametoSlot (Variables|Default|GetSaveGameBP) (Variables|Default|GetSaveGameSlot))
  (Variables|Default|SetGameSlot? true)
  (Development|PrintString "Game Saved"))

(event EventBeginPlay
  (CallFunction|LoadGame))

(fn ConstructionScript)

(fn LoadPlayerParameter
  (bind _savegamebp (Variables|Default|GetSaveGameBP))
  (bind _asbp_player_character_base (Utilities|Casting|CastToBP_PlayerCharacterBase (Game|GetPlayerCharacter 0)))
  (Transformation|SetActorLocation _asbp_player_character_base (Variables|/Game/Commons/SaveLoad/BP_SaveGame.BP_SaveGame_C|GetPlayerLocation (Variables|Default|GetSaveGameBP)) false true)
  (Variables|/Game/Commons/SaveLoad/BP_SaveGame.BP_SaveGame_C|SetPlayer _savegamebp _asbp_player_character_base)
  (Variables|/Game/Commons/SaveLoad/BP_SaveGame.BP_SaveGame_C|SetPrimary%20Weapon _savegamebp (Variables|/Game/Commons/Weapons/Blueprints/BPC_WeaponInventoryComponent.BPC_WeaponInventoryComponent_C|GetPrimaryWeapon (Variables|/Game/Commons/Character/BP_CharacterBase.BP_CharacterBase_C|GetWeaponInventory _asbp_player_character_base)))
  (Variables|/Game/Commons/SaveLoad/BP_SaveGame.BP_SaveGame_C|SetSecondary%20Weapon _savegamebp (Variables|/Game/Commons/Weapons/Blueprints/BPC_WeaponInventoryComponent.BPC_WeaponInventoryComponent_C|GetSecondaryWeapon (Variables|/Game/Commons/Character/BP_CharacterBase.BP_CharacterBase_C|GetWeaponInventory _asbp_player_character_base))))