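; Game instance for Legacy of Time that handles level travel and save slots across Past, Present and Future timelines.
; Saves snapshot the player's class, transform, level and primary and secondary weapons into a GameSaveObject.
; Loading is two-phase: it stores the slot and opens the timeline's level, then OnLevelLoaded applies the data.
; Boss travel saves to a "BossLevel" slot and restores only weapon inventory on arrival.
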(event Custom|OpenNewGame
  (params (Timeline%20To%20load :type E_Timeline%20Enum :default "NewEnumerator0") (SaveSlot :type String))
  (bind _output_get (Variables|Default|SetSaveSlot SaveSlot))
  (bind _output_get_2 (Variables|Default|SetSelectedTimeline Timeline%20To%20load))
  (CallFunction|NewGameSave _output_get)
  (CallFunction|LoadGamefromSaveSlot _output_get _output_get_2))

(event Custom|OnLevelLoaded
  (if (Variables|Default|GetLoadingToBossLevel?)
    (bind _returnvalue (SaveGame|DoesSaveGameExist "BossLevel"))
    (if _returnvalue
      (bind _returnvalue_2 (SaveGame|LoadGamefromSlot "BossLevel"))
      (bind _asgame_save_object (Utilities|Casting|CastToGameSaveObject _returnvalue_2))
      (bind _returnvalue_3 (Actor|GetActorOfClass (.class (Variables|/Game/Commons/Blueprint/GameSaveObject.GameSaveObject_C|GetCharacterData _asgame_save_object))))
      (Utilities|IsValid _returnvalue_3
        (:Is%20Valid
          (Default|LoadWeaponInventory _returnvalue_3 _returnvalue_3 (Variables|/Game/Commons/Blueprint/GameSaveObject.GameSaveObject_C|GetWeaponInventory _asgame_save_object)))))
    (else
      (Game|SetGamePaused true)
      (bind _returnvalue_4 (UserInterface|CreateWidget "/Game/Commons/Widgets/LoadingScreen/WBP_LoadingScreen.WBP_LoadingScreen_C"))
      (Default|FadeOut _returnvalue_4)
      (bind _returnvalue_5 (Actor|GetActorOfClass "/Game/Commons/Character/BP_PlayerCharacterBase.BP_PlayerCharacterBase_C"))
      (Utilities|IsValid _returnvalue_5
        (:Is%20Valid
          (bind _returnvalue_6 (SaveGame|DoesSaveGameExist (Variables|Default|GetLoadSlot)))
          (if _returnvalue_6
            (bind _returnvalue_7 (SaveGame|LoadGamefromSlot (Variables|Default|GetLoadSlot)))
            (bind _asgame_save_object_2 (Utilities|Casting|CastToGameSaveObject _returnvalue_7))
            (Default|LoadSaveData _returnvalue_5 _asgame_save_object_2)
            (else
              (Default|LoadSaveData _returnvalue_5))))))))

(event Custom|SaveGame
  (params (SaveToSlot :type String))
  (bind (_selectedtimeline _savedfromlevel _characterdata _inventorydata) (CallFunction|MakeGameSaveObjectData))
  (bind _output_get (Variables|Default|SetSaveSlot SaveToSlot))
  (bind _returnvalue (SaveGame|DoesSaveGameExist _output_get))
  (if _returnvalue
    (Development|PrintString (Utilities|String|Append "OVERWRITING SAVE SLOT FOR " (Variables|Default|GetSaveSlot)) true true "(R=1.000000,G=0.892180,B=0.000000,A=1.000000)"))
  (bind _returnvalue_2 (SaveGame|CreateSaveGameObject "/Game/Commons/Blueprint/GameSaveObject.GameSaveObject_C"))
  (bind _output_get_2 (Variables|Default|SetAs%20Game%20Save%20Object _returnvalue_2))
  (Variables|Default|SetSelectedTimeline _selectedtimeline)
  (Variables|/Game/Commons/Blueprint/GameSaveObject.GameSaveObject_C|SetLevelName (Variables|Default|GetAs%20Game%20Save%20Object) _savedfromlevel)
  (Variables|/Game/Commons/Blueprint/GameSaveObject.GameSaveObject_C|SetCharacterData (Variables|Default|GetAs%20Game%20Save%20Object) _characterdata)
  (Variables|/Game/Commons/Blueprint/GameSaveObject.GameSaveObject_C|SetWeaponInventory (Variables|Default|GetAs%20Game%20Save%20Object) _inventorydata)
  (bind _returnvalue_3 (SaveGame|SaveGametoSlot _output_get_2 (Variables|Default|GetSaveSlot)))
  (if (not _returnvalue_3)
    (Development|PrintString (Utilities|String|Append "Save failed To: " (Variables|Default|GetSaveSlot)) true true "(R=1.000000,G=0.063810,B=0.000000,A=1.000000)")))

(event Custom|OpenBossLevel
  (params (LevelToOpen :type Soft%20World%20Reference%20Structure))
  (Variables|Default|SetLoadingToBossLevel? true)
  (CallFunction|SaveGame "BossLevel")
  (CallFunction|OpenLevel LevelToOpen))

(event Custom|LoadGameFromSaveSlot
  (params (SaveSlot :type String) (TimelineToLoad :type E_Timeline%20Enum :default "NewEnumerator0"))
  ;[0.15 0.15 0.15 0.5] This only loads the associated level, actual loading of data will be done from the onLevelLoaded
  (Variables|Default|SetLoadSlot SaveSlot)
  (Variables|Default|SetSelectedTimeline TimelineToLoad)
  (switch Utilities|FlowControl|Switch|SwitchonE_Timeline (Variables|Default|GetSelectedTimeline)
    (:NewEnumerator0
      (CallFunction|OpenLevel (Utilities|Struct|MakeSoftWorldReference "/Game/Arbin/PastLevel2.PastLevel2")))
    (:NewEnumerator1
      (CallFunction|OpenLevel (Utilities|Struct|MakeSoftWorldReference "/Game/Krish/Present_Level.Present_Level")))
    (:NewEnumerator2
      (CallFunction|OpenLevel (Utilities|Struct|MakeSoftWorldReference "/Game/SurabGame/Maps/Level_FutureStart.Level_FutureStart")))))

(event Custom|OpenLevel
  (params (LevelToOpen :type Soft%20World%20Reference%20Structure))
  (Game|OpenLevel(byObjectReference) (Utilities|Struct|BreakSoftWorldReference LevelToOpen)))

(fn MakeGameSaveObjectData
  (bind _asbp_player_character_base (Utilities|Casting|CastToBP_PlayerCharacterBase (Game|GetPlayerCharacter 0))
    (:then
      (bind _output_get (LocalVariables|SetCharacter _asbp_player_character_base))
      (bind _weaponinventory (Variables|/Game/Commons/Character/BP_CharacterBase.BP_CharacterBase_C|GetWeaponInventory _output_get)
        (:then
          (LocalVariables|SetWeaponInventory _weaponinventory)
          (Utilities|FlowControl|Sequence
            (:then_0
              ;[0.15 0.15 0.15 0.5] Save primary and secondary weapon if they exist
              (bind _primaryweapon (Variables|/Game/Commons/Weapons/Blueprints/BPC_WeaponInventoryComponent.BPC_WeaponInventoryComponent_C|GetPrimaryWeapon (LocalVariables|GetWeaponInventory))
                (:then
                  (bind _item (CallFunction|MakeInventoryEntry _primaryweapon))
                  (Utilities|Array|AddUnique (LocalVariables|GetInventoryItems) _item))
                (:else)))
            (:then_1
              (bind _secondaryweapon (Variables|/Game/Commons/Weapons/Blueprints/BPC_WeaponInventoryComponent.BPC_WeaponInventoryComponent_C|GetSecondaryWeapon (LocalVariables|GetWeaponInventory))
                (:then
                  (bind _item_2 (CallFunction|MakeInventoryEntry _secondaryweapon))
                  (Utilities|Array|AddUnique (LocalVariables|GetInventoryItems) _item_2))
                (:else)))
            (:then_2
              (bind _returnvalue (Game|GetCurrentLevelName true))
              (return (Variables|Default|GetSelectedTimeline) _returnvalue (Utilities|Struct|MakeS_CharacterData true (Utilities|GetClass (LocalVariables|GetCharacter)) (Transformation|GetActorTransform (LocalVariables|GetCharacter))) (LocalVariables|GetInventoryItems) 0))))
        (:else
          (bind _returnvalue_2 (Game|GetCurrentLevelName true :!label _label))
          (return (Variables|Default|GetSelectedTimeline) _returnvalue_2 "" 0 0))))
    (:CastFailed
      (goto _label))))

(fn MakeInventoryEntry
  (params (Weapon :type BP%20Weapons%20Object%20Reference))
  (bind _weapontype (Variables|/Game/Commons/Weapons/Blueprints/BP_Weapons.BP_Weapons_C|GetWeaponType Weapon))
  (switch Utilities|FlowControl|Switch|SwitchonE_WeaponType _weapontype
    (:NewEnumerator0
      _)
    (:NewEnumerator1
      _)
    (:NewEnumerator2
      (bind _asbp_ranged_weapons (Utilities|Casting|CastToBP_RangedWeapons Weapon)
        (:then
          _)
        (:CastFailed
          _)))
    (:NewEnumerator3
      _))
  (return (Utilities|Struct|MakeS_InventoryItems true (Utilities|GetClass Weapon) (Variables|/Game/Commons/Weapons/Blueprints/BP_Weapons.BP_Weapons_C|GetEquipState Weapon) (Variables|/Game/Commons/Weapons/Blueprints/BP_Weapons.BP_Weapons_C|GetWeaponDamage Weapon) _weapontype (Variables|/Game/Commons/Weapons/Ranged/Bullets/BPC_Magazine.BPC_Magazine_C|GetBulletsCountInMag (Variables|/Game/Commons/Weapons/Ranged/Generic/BP_RangedWeapons.BP_RangedWeapons_C|GetMagazine _asbp_ranged_weapons)) (Variables|/Game/Commons/Weapons/Ranged/Bullets/BPC_Magazine.BPC_Magazine_C|GetRemainingBullets (Variables|/Game/Commons/Weapons/Ranged/Generic/BP_RangedWeapons.BP_RangedWeapons_C|GetMagazine _asbp_ranged_weapons)))))

(fn GetSavedGameDatafromSlot
  (params (SaveSlot :type String))
  (bind _returnvalue (SaveGame|LoadGamefromSlot SaveSlot))
  (bind _asgame_save_object (Utilities|Casting|CastToGameSaveObject _returnvalue))
  (return _asgame_save_object))

(fn NewGameSave
  (params (SlotName :type String))
  (bind (_selectedtimeline _savedfromlevel _characterdata _inventorydata) (CallFunction|MakeGameSaveObjectData))
  (SaveGame|DeleteGameinSlot SlotName)
  (bind _returnvalue (SaveGame|CreateSaveGameObject "/Game/Commons/Blueprint/GameSaveObject.GameSaveObject_C"))
  (Variables|/Game/Commons/Blueprint/GameSaveObject.GameSaveObject_C|SetSelectedTimeline _returnvalue _selectedtimeline)
  (Variables|/Game/Commons/Blueprint/GameSaveObject.GameSaveObject_C|SetLevelName _returnvalue _savedfromlevel)
  (Variables|/Game/Commons/Blueprint/GameSaveObject.GameSaveObject_C|SetCharacterData _returnvalue _characterdata)
  (Variables|/Game/Commons/Blueprint/GameSaveObject.GameSaveObject_C|SetWeaponInventory _returnvalue _inventorydata)
  (bind _returnvalue_2 (SaveGame|SaveGametoSlot _returnvalue SlotName))
  (if _returnvalue_2
    (Development|PrintString (Utilities|String|Append "New game saved " (Variables|Default|GetSaveSlot)))
    (else
      (Development|PrintString (Utilities|String|Append "New game save failed" (Variables|Default|GetSaveSlot)) true true "(R=1.000000,G=0.061379,B=0.000000,A=1.000000)"))))