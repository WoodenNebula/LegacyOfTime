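; Boss arena gate actor that opens while its Box trigger is overlapped and closes when an overlap ends.
; BeginPlay stores the Gate component's relative location as the closed position and sets the OpenGate timeline's play rate from AnimSpeed.
; Overlap begin and end play and reverse the timeline, whose Height track lerps the gate between its closed and open offsets.
; Neither overlap event filters which actor triggers it.
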(event OnComponentBeginOverlap(Box)
  (params (OverlappedComponent :type Primitive%20Component%20Object%20Reference) (OtherActor :type Actor%20Object%20Reference) (OtherComp :type Primitive%20Component%20Object%20Reference) (OtherBodyIndex :type Integer) (bFromSweep :type Boolean) (SweepResult :type Hit%20Result%20Structure%20%28by%20ref%29))
  (bind _height (Timeline|OpenGate Play)
    (:Update
      (Transformation|SetRelativeLocation (Variables|Default|GetGate) (Math|Vector|Lerp(Vector) (Variables|Default|GetOffsetClose) (Variables|Default|GetOffsetOpen) _height) false false))))

(event OnComponentEndOverlap(Box)
  (params (OverlappedComponent :type Primitive%20Component%20Object%20Reference) (OtherActor :type Actor%20Object%20Reference) (OtherComp :type Primitive%20Component%20Object%20Reference) (OtherBodyIndex :type Integer))
  (bind _height (Timeline|OpenGate Reverse)
    (:Update
      (Transformation|SetRelativeLocation (Variables|Default|GetGate) (Math|Vector|Lerp(Vector) (Variables|Default|GetOffsetClose) (Variables|Default|GetOffsetOpen) _height) false false))))

(event EventBeginPlay
  (Variables|Default|SetOffsetClose (.location (Transformation|GetRelativeTransform (Variables|Default|GetGate))))
  (Components|Timeline|SetPlayRate (Variables|Default|GetOpenGate) (Variables|Default|GetAnimSpeed)))

(fn ConstructionScript)