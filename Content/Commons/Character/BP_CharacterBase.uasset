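; Base character Blueprint for both player and NPCs, tagged by controller at BeginPlay, handling movement, health and weapon use.
; Input handlers set sprint and jump, and pass weapon actions to WeaponInventory, gated on HealthComponent's death state.
; Combat notify interface events relay to the inventory, while damage interface calls feed HealthComponent.
; Death state changes fire start and finish hooks and release any active ranged aim or fire.
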(event Custom|OnDeathStarted)

(event Custom|OnDeathFinished)

(event Custom|OnCharacterDeathStateChanged
  (params (NewState :type E_DeathState%20Enum :default "NewEnumerator0"))
  (switch Utilities|FlowControl|Switch|SwitchonE_DeathState NewState
    (:NewEnumerator1
      (CallFunction|OnDeathStarted))
    (:NewEnumerator2
      (CallFunction|OnDeathFinished)))
  (Utilities|FlowControl|Sequence
    (:then_0
      (if (CallFunction|IsAiming?)
        (Default|HandleAimEnd (Variables|WeaponInventory|GetWeaponInventory))))
    (:then_1
      (if (CallFunction|IsHoldingFire?)
        (Default|HandleAttackCompleteInput (Variables|WeaponInventory|GetWeaponInventory))))))

(event EventBeginPlay
  (bind _tags (Variables|Actor|GetTags))
  (if (Pawn|IsPlayerControlled)
    (Utilities|Array|Add _tags "Player")
    (else
      (Utilities|Array|Add _tags "NPC")))
  (Utilities|FlowControl|Sequence
    (:then_0
      (CallFunction|InitMovement))
    (:then_1
      (CallFunction|ChangeIdleAnimation (Variables|Animation|GetDefaultIdleAnimationSequence)))
    (:then_2
      (Utilities|FlowControl|DelayUntilNextTick)
      (Default|Init (Variables|Default|GetHealthComponent))
      (Default|Init (Variables|WeaponInventory|GetWeaponInventory))
      (EventDispatchers|BindEventtoOnDeathStateChanged (Variables|Default|GetHealthComponent) (EventDispatchers|CreateEvent :!event Custom|OnCharacterDeathStateChanged)))))

(event Custom|HandleSprintReleaseInput
  ;[0.15 0.15 0.15 0.5] Movement Inputs
  (Variables|Movement|SetIsSprinting false)
  (Variables|/Script/Engine.CharacterMovementComponent|SetMaxWalkSpeed (Variables|Character|GetCharacterMovement) (Variables|Movement|GetWalkSpeed)))

(event Custom|HandleAttackCompleteInput
  ;[0.15 0.15 0.15 0.5] Weapon Inputs
  (Variables|Default|SetbIsAttackDown false)
  (if (CallFunction|IsAlive)
    (Default|HandleAttackCompleteInput (Variables|WeaponInventory|GetWeaponInventory))))

(event Custom|HandleAimCompleteInput
  ;[0.15 0.15 0.15 0.5] Weapon Inputs
  (Variables|Default|SetbIsAimDown false)
  (if (CallFunction|IsAlive)
    (Default|HandleAimEnd (Variables|WeaponInventory|GetWeaponInventory))
    (Development|PrintString "AimUp" true true "(R=1.000000,G=0.000000,B=0.149053,A=1.000000)")))

(event Custom|HandleAimStartInput
  ;[0.15 0.15 0.15 0.5] Weapon Inputs
  (Variables|Default|SetbIsAimDown true)
  (if (CallFunction|IsAlive)
    (Default|HandleAimStart (Variables|WeaponInventory|GetWeaponInventory))
    (Development|PrintString "AimDown" true true "(R=0.000000,G=1.000000,B=0.111461,A=1.000000)")
    (else
      (CallFunction|HandleAimCompleteInput))))

(event Custom|HandleAttackStartInput
  ;[0.15 0.15 0.15 0.5] Weapon Inputs
  (Variables|Default|SetbIsAttackDown true)
  (if (CallFunction|IsAlive)
    (Default|HandleAttackStartInput (Variables|WeaponInventory|GetWeaponInventory))
    (else
      (CallFunction|HandleAttackCompleteInput))))

(event Custom|HandleThrowableSelectInput
  ;[0.15 0.15 0.15 0.5] Weapon Inputs
  (if (CallFunction|IsAlive)
    (Default|HandleThrowableSelect (Variables|WeaponInventory|GetWeaponInventory))))

(event Custom|HandleJumpCompleteInput
  ;[0.15 0.15 0.15 0.5] Movement Inputs
  (Character|StopJumping))

(event Custom|HandleJumpTriggerInput
  ;[0.15 0.15 0.15 0.5] Movement Inputs
  (Character|Jump))

(event Custom|HandlePrimaryWeaponSelectInput
  ;[0.15 0.15 0.15 0.5] Weapon Inputs
  (if (CallFunction|IsAlive)
    (Default|HandlePrimaryWeaponSelect (Variables|WeaponInventory|GetWeaponInventory))))

(event Custom|HandleSprintStartInput
  ;[0.15 0.15 0.15 0.5] Movement Inputs
  (Variables|Movement|SetIsSprinting true)
  (Variables|/Script/Engine.CharacterMovementComponent|SetMaxWalkSpeed (Variables|Character|GetCharacterMovement) (Variables|Movement|GetSprintSpeed)))

(event Custom|HandleSecondaryWeaponSelectInput
  ;[0.15 0.15 0.15 0.5] Weapon Inputs
  (if (CallFunction|IsAlive)
    (Default|HandleSecondaryWeaponSelect (Variables|WeaponInventory|GetWeaponInventory))))

(event Custom|HandleReloadInput
  ;[0.15 0.15 0.15 0.5] Weapon Inputs
  (if (CallFunction|IsAlive)
    (Default|HandleReload (Variables|WeaponInventory|GetWeaponInventory))))

(event EventRecieveReloadNotify
  ;[0.15 0.15 0.15 0.5] Ranged Weapon Notify Handles
  (Default|OnWeaponReloadCompleteNotifyRecieved (Variables|WeaponInventory|GetWeaponInventory)))

(event EventRecieveComboStopNotify
  (Default|OnComboStopNotifyRecieved (Variables|WeaponInventory|GetWeaponInventory)))

(event EventRecieveComboNextNotify
  (Default|OnComboNextNotifyRecieved (Variables|WeaponInventory|GetWeaponInventory)))

(event EventRecieveWeaponUnequippedNotify
  ;[0.15 0.15 0.15 0.5] Generic Weapon Notify Handles
  (Default|OnWeaponUnattachedNotifyRecieved (Variables|WeaponInventory|GetWeaponInventory)))

(event EventRecieveProjectileFiredNotify
  ;[0.15 0.15 0.15 0.5] Ranged Weapon Notify Handles
  (Default|OnProjectileFiredNotifyRecieved (Variables|WeaponInventory|GetWeaponInventory)))

(event EventRecieveWeaponEquippedNotify
  ;[0.15 0.15 0.15 0.5] Generic Weapon Notify Handles
  (Default|OnWeaponAttachedNotifyRecieved (Variables|WeaponInventory|GetWeaponInventory)))

(event EventRecieveAttackedNotify
  (Default|OnAttackedNotifyRecieved (Variables|WeaponInventory|GetWeaponInventory)))

(event EventTakeDamage
  (params (DamageValue :type Integer) (IsStunned :type Boolean) (StunTime :type Float%20%28double-precision%29) (ImpactPoint :type Vector :default "0, 0, 0") (ImpactNormal :type Vector :default "0, 0, 0") (HitFromDirection :type E_HitFromDirection%20Enum :default "NewEnumerator6"))
  (Development|PrintString (Utilities|String|Append "Damaged:" (Utilities|String|ToString(Integer) DamageValue)) true true "(R=1.000000,G=0.031389,B=0.000000,A=1.000000)")
  (Default|Damage (Variables|Default|GetHealthComponent) DamageValue IsStunned StunTime))

(event EventANPlayerDied
  (Default|FinishDeath (Variables|Default|GetHealthComponent)))

(fn ConstructionScript)

(fn ChangeIdleAnimation
  (params (NewIdleLoopAnimSequence :type Anim%20Sequence%20Object%20Reference))
  (Utilities|IsValid NewIdleLoopAnimSequence
    (:Is%20Valid
      (Variables|Animation|SetIdleAnimationSequence NewIdleLoopAnimSequence))
    (:Is%20Not%20Valid
      (Variables|Animation|SetIdleAnimationSequence (Variables|Animation|GetDefaultIdleAnimationSequence)))))

(fn IsAlive
  (bind _healthcomponent (Variables|Default|GetHealthComponent)
    (:then
      (return (Utilities|Enum|Equal(Enum) (Variables|/Game/Commons/Blueprint/BPC_HealthComponent.BPC_HealthComponent_C|GetDeathState _healthcomponent) "NewEnumerator0")))
    (:else
      (return false))))

(fn InitMovement
  (Variables|/Script/Engine.CharacterMovementComponent|SetCrouchedHalfHeight (Variables|Character|GetCharacterMovement) (Variables|Default|GetCrouchingCapsuleHeight))
  (Variables|/Script/Engine.CharacterMovementComponent|SetMaxWalkSpeed (Variables|Character|GetCharacterMovement) (Variables|Movement|GetWalkSpeed))
  (Variables|/Script/Engine.CharacterMovementComponent|SetMaxWalkSpeedCrouched (Variables|Character|GetCharacterMovement) (Variables|Movement|GetCrouchWalkSpeed)))

(fn IsPlayerCharacter?
  (return (Actor|ActorHasTag "Player")))

(fn IsAiming?
  (bind _weaponinventory (Variables|WeaponInventory|GetWeaponInventory)
    (:then
      (bind _selectedweapon (Variables|/Game/Commons/Weapons/Blueprints/BPC_WeaponInventoryComponent.BPC_WeaponInventoryComponent_C|GetSelectedWeapon _weaponinventory)
        (:then
          (if (GameplayTags|MatchesTag (Variables|/Game/Commons/Weapons/Blueprints/BP_Weapons.BP_Weapons_C|GetWeaponTypeTag _selectedweapon) "(TagName=\"Weapon.Type.Ranged\")")
            (bind _isaiming (Class|BPIRangedWeaponInterface|IsAiming(Message) (Variables|/Game/Commons/Weapons/Blueprints/BPC_WeaponInventoryComponent.BPC_WeaponInventoryComponent_C|GetSelectedWeapon (Variables|WeaponInventory|GetWeaponInventory))))
            (return _isaiming)
            (else
              _)))
        (:else
          _))
      (return false))
    (:else)))

(fn IsHoldingFire?
  (bind _weaponinventory (Variables|WeaponInventory|GetWeaponInventory)
    (:then
      (bind _selectedweapon (Variables|/Game/Commons/Weapons/Blueprints/BPC_WeaponInventoryComponent.BPC_WeaponInventoryComponent_C|GetSelectedWeapon _weaponinventory)
        (:then
          (if (GameplayTags|MatchesTag (Variables|/Game/Commons/Weapons/Blueprints/BP_Weapons.BP_Weapons_C|GetWeaponTypeTag _selectedweapon) "(TagName=\"Weapon.Type.Ranged\")")
            (bind _isholdingfire_ (Class|BPIRangedWeaponInterface|IsHoldingFire(Message) (Variables|/Game/Commons/Weapons/Blueprints/BPC_WeaponInventoryComponent.BPC_WeaponInventoryComponent_C|GetSelectedWeapon (Variables|WeaponInventory|GetWeaponInventory))))
            (return _isholdingfire_)
            (else
              _)))
        (:else
          _))
      (return false))
    (:else)))

(fn WantstoAttack?
  (return (Variables|Default|GetbIsAttackDown)))

(fn WantstoAim?
  (return (Variables|Default|GetbIsAimDown)))