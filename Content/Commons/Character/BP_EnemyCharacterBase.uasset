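; Base enemy character Blueprint that adds a health bar and death cleanup to its parent character class.
; On BeginPlay it creates a WBP_EnemyHealthbar, then a tick later binds it to the HealthComponent, hides it and assigns it to the Widget component.
; Death start destroys that component and hides the bar.
; Death finish starts a randomized timer that destroys the actor after a few seconds.
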(event Custom|DestroySelf
  (Actor|DestroyActor))

(event EventOnDeathStarted
  (|CallParentFunction)
  (Components|DestroyComponent (Variables|Default|GetWidget))
  (Default|Hide (Variables|Default|GetHealthBar)))

(event EventOnDeathFinished
  (|CallParentFunction)
  (Utilities|Time|SetTimerbyEvent (delegate Custom|DestroySelf) (Math|Random|RandomFloatinRange 5.0 1e+01)))

(event EventBeginPlay
  (|CallParentFunction)
  (bind _returnvalue (UserInterface|CreateWidget "/Game/Commons/Widgets/WBP_EnemyHealthbar.WBP_EnemyHealthbar_C"))
  (bind _output_get (Variables|Default|SetHealthBar _returnvalue))
  (Utilities|FlowControl|DelayUntilNextTick)
  (Default|Init _output_get (Variables|Default|GetHealthComponent))
  (Default|Hide _output_get)
  (UserInterface|SetWidget (Variables|Default|GetWidget) (Variables|Default|GetHealthBar)))

(fn ConstructionScript)