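; Character weapon inventory component that holds a primary, secondary and throwable weapon and destroys them with the owner.
; It forwards attack, aim, reload and animation notify events to the selected weapon.
; Equip and unequip toggles follow a switch state reported by each weapon, finish on attach notifies and update owner gameplay tags.
; Switching directly between equipped weapons is unwired: the unequip branch never runs and the queued type is never set.
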(event Custom|HandleAttackStartInput
  ;[0.15 0.15 0.15 0.5] Attack Inputs
  (bind _selectedweapon (Variables|WeaponInventory:Inventory|GetSelectedWeapon)
    (:then
      (Default|OnAttackInputStarted _selectedweapon))
    (:else)))

(event Custom|HandleAttackCompleteInput
  ;[0.15 0.15 0.15 0.5] Attack Inputs
  (bind _selectedweapon (Variables|WeaponInventory:Inventory|GetSelectedWeapon)
    (:then
      (Default|OnAttackInputReleased _selectedweapon))
    (:else)))

(event Custom|HandleReload
  (bind _selectedweapon (Variables|WeaponInventory:Inventory|GetSelectedWeapon)
    (:then
      (switch Utilities|FlowControl|Switch|SwitchonE_WeaponType (Variables|/Game/Commons/Weapons/Blueprints/BP_Weapons.BP_Weapons_C|GetWeaponType _selectedweapon)
        (:NewEnumerator1
          (Development|PrintString "Cannot Reload Selected Weapon" true true "(R=1.000000,G=0.143594,B=0.000000,A=1.000000)" :!label _label))
        (:NewEnumerator2
          (Class|BPIRangedWeaponInterface|Reload(Message) (Variables|WeaponInventory:Inventory|GetSelectedWeapon)))
        (:NewEnumerator3
          (goto _label))))
    (:else
      (Development|PrintString "Invalid Selected Weapon" true true "(R=1.000000,G=0.143594,B=0.000000,A=1.000000)"))))

(event Custom|Init
  ;[0.15 0.15 0.15 0.5] Set player owner reference
  (bind _asbp_character_base (Utilities|Casting|CastToBP_CharacterBase (Components|GetOwner)))
  (bind _output_get (Variables|WeaponInventory:States|SetOwner _asbp_character_base))
  (Game|AssignOnDestroyed _output_get (delegate Custom|Destroy%20All%20Inventory%20Objects)))

(event Custom|HandleAimStart
  (bind _selectedweapon (Variables|WeaponInventory:Inventory|GetSelectedWeapon)
    (:then
      (switch Utilities|FlowControl|Switch|SwitchonE_WeaponType (Variables|/Game/Commons/Weapons/Blueprints/BP_Weapons.BP_Weapons_C|GetWeaponType _selectedweapon)
        (:NewEnumerator2
          (Class|BPIRangedWeaponInterface|OnAimBegin(Message) (Variables|WeaponInventory:Inventory|GetSelectedWeapon)))))
    (:else)))

(event Custom|Destroy%20All%20Inventory%20Objects
  (params (DestroyedActor :type Actor%20Object%20Reference))
  (Utilities|FlowControl|Sequence
    (:then_0
      (bind _primaryweapon (Variables|WeaponInventory:Inventory|GetPrimaryWeapon)
        (:then
          (Actor|DestroyActor _primaryweapon))
        (:else)))
    (:then_1
      (bind _secondaryweapon (Variables|WeaponInventory:Inventory|GetSecondaryWeapon)
        (:then
          (Actor|DestroyActor _secondaryweapon))
        (:else)))
    (:then_2
      (bind _throwable (Variables|WeaponInventory:Inventory|GetThrowable)
        (:then
          (Actor|DestroyActor _throwable))
        (:else)))
    (:then_3
      (bind _selectedweapon (Variables|WeaponInventory:Inventory|GetSelectedWeapon)
        (:then
          (Actor|DestroyActor _selectedweapon))
        (:else)))))

(event Custom|HandleAimEnd
  (bind _selectedweapon (Variables|WeaponInventory:Inventory|GetSelectedWeapon)
    (:then
      (switch Utilities|FlowControl|Switch|SwitchonE_WeaponType (Variables|/Game/Commons/Weapons/Blueprints/BP_Weapons.BP_Weapons_C|GetWeaponType _selectedweapon)
        (:NewEnumerator2
          (Class|BPIRangedWeaponInterface|OnAimEnd(Message) (Variables|WeaponInventory:Inventory|GetSelectedWeapon)))))
    (:else)))

(event Custom|OnWeaponReloadCompleteNotifyRecieved
  (bind _selectedweapon (Variables|WeaponInventory:Inventory|GetSelectedWeapon)
    (:then
      (Class|BPICombatNotifyRecievable|RecieveReloadNotify(Message) _selectedweapon))
    (:else)))

(event Custom|OnAttackedNotifyRecieved
  (bind _selectedweapon (Variables|WeaponInventory:Inventory|GetSelectedWeapon)
    (:then
      (Class|BPICombatNotifyRecievable|RecieveAttackedNotify(Message) _selectedweapon))
    (:else)))

(event Custom|OnComboNextNotifyRecieved
  (bind _selectedweapon (Variables|WeaponInventory:Inventory|GetSelectedWeapon)
    (:then
      (Class|BPICombatNotifyRecievable|RecieveComboNextNotify(Message) _selectedweapon))
    (:else)))

(event Custom|OnWeaponAttachedNotifyRecieved
  (bind _weapontotoggle (Variables|WeaponInventory:States|GetWeaponToToggle)
    (:then
      ;[0.15 0.15 0.15 0.5] Update Weapon Inventory States
      (bind _output_get (Variables|WeaponInventory:Inventory|SetSelectedWeapon _weapontotoggle))
      (Variables|WeaponInventory:States|SetSelectedWeaponType (Variables|/Game/Commons/Weapons/Blueprints/BP_Weapons.BP_Weapons_C|GetWeaponPriorityType _output_get))
      ;[0.15 0.15 0.15 0.5] Complete Weapon Equiption
      (Class|BPICombatNotifyRecievable|RecieveWeaponEquippedNotify(Message) (Variables|WeaponInventory:Inventory|GetSelectedWeapon))
      (Variables|WeaponInventory:States|SetWeaponToToggle 0)
      (Variables|WeaponInventory:States|SetQueuedWeaponType "NewEnumerator0"))
    (:else)))

(event Custom|OnComboStopNotifyRecieved
  (bind _selectedweapon (Variables|WeaponInventory:Inventory|GetSelectedWeapon)
    (:then
      (Class|BPICombatNotifyRecievable|RecieveComboStopNotify(Message) _selectedweapon))
    (:else)))

(event Custom|OnWeaponUnattachedNotifyRecieved
  (Variables|WeaponInventory:Inventory|GetSelectedWeapon
    (:then
      ;[0.15 0.15 0.15 0.5] Update Weapon Inventory States
      (Variables|WeaponInventory:Inventory|SetSelectedWeapon 0)
      (Variables|WeaponInventory:States|SetSelectedWeaponType "NewEnumerator0")
      ;[0.15 0.15 0.15 0.5] Complete Weapon Unequiption
      (Class|BPICombatNotifyRecievable|RecieveWeaponUnequippedNotify(Message) (Variables|WeaponInventory:States|GetWeaponToToggle))
      (Variables|WeaponInventory:States|SetWeaponToToggle 0)
      (switch Utilities|FlowControl|Switch|SwitchonE_WeaponPriorityType (Variables|WeaponInventory:States|GetQueuedWeaponType)
        (:NewEnumerator1
          (CallFunction|HandlePrimaryWeaponSelect))
        (:NewEnumerator2
          (CallFunction|HandleSecondaryWeaponSelect))
        (:NewEnumerator3
          (CallFunction|HandleThrowableSelect))))
    (:else)))

(event Custom|OnProjectileFiredNotifyRecieved
  (bind _selectedweapon (Variables|WeaponInventory:Inventory|GetSelectedWeapon)
    (:then
      (Class|BPICombatNotifyRecievable|RecieveProjectileFiredNotify(Message) _selectedweapon))
    (:else)))

(event Custom|HandlePrimaryWeaponSelect
  (Variables|WeaponInventory:States|SetWeaponToToggle (Variables|WeaponInventory:Inventory|GetPrimaryWeapon))
  (CallFunction|ToggleWeapon))

(event Custom|HandleSecondaryWeaponSelect
  (Variables|WeaponInventory:States|SetWeaponToToggle (Variables|WeaponInventory:Inventory|GetSecondaryWeapon))
  (CallFunction|ToggleWeapon))

(event Custom|ToggleWeapon
  (switch Utilities|FlowControl|Switch|SwitchonE_WeaponEquipState (Variables|WeaponInventory:States|GetWeaponSwitchState)
    (:NewEnumerator0
      ;[0.15 0.15 0.15 0.5] Unequipped means target weapon can be simply equipped
      (bind _weapontotoggle (Variables|WeaponInventory:States|GetWeaponToToggle)
        (:then
          (Default|OnInitiateEquip _weapontotoggle))
        (:else)))
    (:NewEnumerator1
      (Development|PrintString "Equiping another weapon" true true "(R=1.000000,G=0.788008,B=0.000000,A=1.000000)" :!label _label))
    (:NewEnumerator2
      (goto _label))
    (:NewEnumerator4
      (goto _label))
    (:NewEnumerator3
      (bind _weapontotoggle_2 (Variables|WeaponInventory:States|GetWeaponToToggle)
        (:then
          (if (Utilities|Enum|Equal(Enum) (Variables|WeaponInventory:States|GetSelectedWeaponType) (Variables|/Game/Commons/Weapons/Blueprints/BP_Weapons.BP_Weapons_C|GetWeaponPriorityType _weapontotoggle_2))
            ;[0.15 0.15 0.15 0.5] If request is to toggle already selected weapon, unequip it
            (Default|OnInitiateUnequip (Variables|WeaponInventory:States|GetWeaponToToggle))))
        (:else)))))

(event Custom|HandleThrowableSelect
  (Variables|WeaponInventory:States|SetWeaponToToggle (Variables|WeaponInventory:Inventory|GetThrowable))
  (CallFunction|ToggleWeapon))

(event Custom|OnWeaponSwitchingStateUpdated
  (params (NewState :type E_WeaponEquipState%20Enum :default "NewEnumerator0"))
  ;[0.15 0.15 0.15 0.5] ToggleWeaponStateUpdate
  (bind _output_get (Variables|WeaponInventory:States|SetWeaponSwitchState NewState))
  (switch Utilities|FlowControl|Switch|SwitchonE_WeaponEquipState _output_get
    (:NewEnumerator4
      (GameplayTags|RemoveGameplayTag (Variables|/Game/Commons/Character/BP_CharacterBase.BP_CharacterBase_C|GetGameplayTags (Variables|WeaponInventory:States|GetOwner)) (Variables|/Game/Commons/Weapons/Blueprints/BP_Weapons.BP_Weapons_C|GetWeaponTypeTag (Variables|WeaponInventory:Inventory|GetSelectedWeapon)) :!class /Script/GameplayTags.BlueprintGameplayTagLibrary))
    (:NewEnumerator3
      (GameplayTags|AddGameplayTag (Variables|/Game/Commons/Character/BP_CharacterBase.BP_CharacterBase_C|GetGameplayTags (Variables|WeaponInventory:States|GetOwner)) (Variables|/Game/Commons/Weapons/Blueprints/BP_Weapons.BP_Weapons_C|GetWeaponTypeTag (Variables|WeaponInventory:Inventory|GetSelectedWeapon)) :!class /Script/GameplayTags.BlueprintGameplayTagLibrary))))

(fn TryAddWeapontoInventory
  (params (Weapon :type BP%20Weapons%20Object%20Reference))
  (Utilities|IsValid Weapon
    (:Is%20Valid
      (bind _output_get (LocalVariables|SetTargetWeapon Weapon))
      (switch Utilities|FlowControl|Switch|SwitchonE_WeaponPriorityType (Variables|/Game/Commons/Weapons/Blueprints/BP_Weapons.BP_Weapons_C|GetWeaponPriorityType _output_get)
        (:NewEnumerator1
          ;[0.15 0.15 0.15 0.5] Does the priority type of weapon(primary, secondary) already exist?
          (Variables|WeaponInventory:Inventory|GetPrimaryWeapon
            (:then
              _)
            (:else
              ;[0.0246 0.15 0 0.5] Can Add the Weapon
              (Variables|WeaponInventory:Inventory|SetPrimaryWeapon (LocalVariables|GetTargetWeapon))
              (EventDispatchers|BindEventtoOnWeaponSwitchStateUpdated (LocalVariables|GetTargetWeapon) (EventDispatchers|CreateEvent :!event Custom|OnWeaponSwitchingStateUpdated) :!label _label)
              (return true))))
        (:NewEnumerator2
          (Variables|WeaponInventory:Inventory|GetSecondaryWeapon
            (:then
              _)
            (:else
              ;[0.0246 0.15 0 0.5] Can Add the Weapon
              (Variables|WeaponInventory:Inventory|SetSecondaryWeapon (LocalVariables|GetTargetWeapon))
              (goto _label))))
        (:NewEnumerator3
          (Variables|WeaponInventory:Inventory|GetThrowable
            (:then
              _)
            (:else
              ;[0.15 0.1324 0 0.5] Projectile Doesnt Exist already
              (bind _asbp_throwables (Utilities|Casting|CastToBP_Throwables (LocalVariables|GetTargetWeapon)))
              (bind _output_get_2 (Variables|WeaponInventory:Inventory|SetThrowable _asbp_throwables))
              (EventDispatchers|BindEventtoOnWeaponSwitchStateUpdated _output_get_2 (EventDispatchers|CreateEvent :!event Custom|OnWeaponSwitchingStateUpdated))))
          (bind _success_ (Default|TryAddThrowable (Variables|WeaponInventory:Inventory|GetThrowable)))
          (if _success_
            (return true)
            (else
              (return false)))))
      ;[0.15 0 0 0.5] Weapon Already Exists
      (Development|PrintString "Weapon Already Exists" true true "(R=1.000000,G=0.000000,B=0.019754,A=1.000000)")
      (return false))
    (:Is%20Not%20Valid
      (Development|PrintString "Invalid Weapon" true true "(R=1.000000,G=0.013236,B=0.000000,A=1.000000)")
      (return false))))