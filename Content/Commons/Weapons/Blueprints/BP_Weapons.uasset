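; Base weapon actor that characters can pick up, equip, unequip and attack with.
; Sphere overlap binds the character's interaction event; pickup adds it to the inventory, attaches it and looks up montages by weapon type tag.
; Equip and unequip play montages through an equip state, with anim-notify interface events swapping sockets and idle animation.
; Attack fires on input press or release and plays the first attack montage, gated by an always-true CanAttack.
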(event Custom|OnAttackInputStarted
  ;[0.15 0.15 0.15 0.5] Attack event inputs
  (if (Variables|Default|GetShould%20Attack%20Trigger%20on%20Input%20Start?)
    (CallFunction|OnAttackRequest)))

(event Custom|Force%20Equip
  (Transformation|AttachComponentToComponent (Variables|Default|GetSkeletalMesh) (Variables|/Script/Engine.Character|GetMesh (Variables|InventoryState|GetOwnerCharacter)) (.equipped (.SocketToAttachTo (Utilities|Struct|BreakS_WeaponAnimations (Variables|Animation|GetWeaponMontages)))) "SnapToTarget" "SnapToTarget" "SnapToTarget" true))

(event Custom|ForceUnequip
  (Transformation|AttachComponentToComponent (Variables|Default|GetSkeletalMesh) (Variables|/Script/Engine.Character|GetMesh (Variables|InventoryState|GetOwnerCharacter)) (.unequipped (.SocketToAttachTo (Utilities|Struct|BreakS_WeaponAnimations (Variables|Animation|GetWeaponMontages)))) "SnapToTarget" "SnapToTarget" "SnapToTarget" true))

(event Custom|OnAttackInputReleased
  ;[0.15 0.15 0.15 0.5] Attack event inputs
  (if (not (Variables|Default|GetShould%20Attack%20Trigger%20on%20Input%20Start?))
    (CallFunction|OnAttackRequest)))

(event Custom|OnInitiateUnequip
  ;[0.15 0.15 0.15 0.5] Play Weapon Unequip Animation if valid
  (if (and (Variables|InventoryState|GetHasBeenPickedUp) (Utilities|Enum|Equal(Enum) (Variables|InventoryState|GetEquipState) "NewEnumerator3"))
    (Utilities|FlowControl|Sequence
      (:then_0
        (bind _output_get (Variables|InventoryState|SetEquipState "NewEnumerator4"))
        (Default|CallOnWeaponSwitchStateUpdated _output_get))
      (:then_1
        (Animation|Montage|PlayMontage (Variables|/Script/Engine.Character|GetMesh (Variables|InventoryState|GetOwnerCharacter)) (.unequip (Variables|Animation|GetWeaponMontages))
          (:OnCompleted
            _)
          (:OnInterrupted
            _))
        (bind _output_get_2 (Variables|InventoryState|SetEquipState "NewEnumerator0"))
        (Default|CallOnWeaponSwitchStateUpdated _output_get_2)
        (CallFunction|ForceUnequip)))))

(event Custom|OnInitiateEquip
  ;[0.15 0.15 0.15 0.5] Play Weapon Equip Animation if valid
  (if (and (Variables|InventoryState|GetHasBeenPickedUp) (Utilities|Enum|Equal(Enum) (Variables|InventoryState|GetEquipState) "NewEnumerator0"))
    (Utilities|FlowControl|Sequence
      (:then_0
        (bind _output_get (Variables|InventoryState|SetEquipState "NewEnumerator1"))
        (Default|CallOnWeaponSwitchStateUpdated _output_get))
      (:then_1
        (Animation|Montage|PlayMontage (Variables|/Script/Engine.Character|GetMesh (Variables|InventoryState|GetOwnerCharacter)) (.equip (Variables|Animation|GetWeaponMontages))
          (:OnCompleted
            _)
          (:OnInterrupted
            _))
        (bind _output_get_2 (Variables|InventoryState|SetEquipState "NewEnumerator3"))
        (Default|CallOnWeaponSwitchStateUpdated _output_get_2)
        (CallFunction|ForceEquip)))))

(event Custom|OnAttackRequest
  ;[0.15 0.15 0.15 0.5] Attack event inputs
  (bind _bcanattack (CallFunction|CanAttack))
  (if _bcanattack
    (CallFunction|InitiateAttack)))

(event OnComponentEndOverlap(Sphere)
  (params (OverlappedComponent :type Primitive%20Component%20Object%20Reference) (OtherActor :type Actor%20Object%20Reference) (OtherComp :type Primitive%20Component%20Object%20Reference) (OtherBodyIndex :type Integer))
  ;[0 0 0 0.5] Interactable Area Enter and Exit
  (CallFunction|HandlePlayerExitsCollision OtherActor))

(event OnComponentBeginOverlap(Sphere)
  (params (OverlappedComponent :type Primitive%20Component%20Object%20Reference) (OtherActor :type Actor%20Object%20Reference) (OtherComp :type Primitive%20Component%20Object%20Reference) (OtherBodyIndex :type Integer) (bFromSweep :type Boolean) (SweepResult :type Hit%20Result%20Structure%20%28by%20ref%29))
  ;[0 0 0 0.5] Interactable Area Enter and Exit
  (CallFunction|HandlePlayerEntersCollision OtherActor))

(event Custom|HandlePlayerExitsCollision
  (params (Actor :type Actor%20Object%20Reference))
  ;[0.1343 0.15 0.1357 0.5] Interactable Area Handles
  (Variables|InventoryState|GetOwnerCharacter
    (:then
      _)
    (:else
      (bind _asbp_character_base (Utilities|Casting|CastToBP_CharacterBase Actor))
      (Variables|InventoryState|SetOwnerCharacter _asbp_character_base)))
  (EventDispatchers|UnbindEventfromOnInteractionTriggered (Variables|InventoryState|GetOwnerCharacter) (EventDispatchers|CreateEvent :!event Custom|HandleOnInteract)))

(event Custom|HandlePlayerEntersCollision
  (params (Actor :type Actor%20Object%20Reference))
  ;[0.1343 0.15 0.1357 0.5] Interactable Area Handles
  (bind _shouldinteract_ (CallFunction|ShouldInteract))
  (if _shouldinteract_
    (Variables|InventoryState|GetOwnerCharacter
      (:then
        _)
      (:else
        (bind _asbp_character_base (Utilities|Casting|CastToBP_CharacterBase Actor))
        (Variables|InventoryState|SetOwnerCharacter _asbp_character_base)))
    (EventDispatchers|AssignOnInteractionTriggered (Variables|InventoryState|GetOwnerCharacter) (EventDispatchers|CreateEvent :!event Custom|HandleOnInteract))))

(event Custom|OnWeaponPickedUp
  (params (PickedBy :type BP%20Character%20Base%20Object%20Reference))
  (Utilities|FlowControl|Sequence
    (:then_0
      ;[0.15 0.15 0.15 0.5] Execute pickup logic
      (bind _output_get (Variables|InventoryState|SetOwnerCharacter PickedBy))
      (Transformation|AttachComponentToComponent (Variables|/Script/Engine.Character|GetMesh _output_get) (.unequipped (Variables|Config|GetWeaponSockets)) "SnapToTarget" "SnapToTarget" "SnapToTarget" true)
      (Variables|InventoryState|SetHasBeenPickedUp true)
      (Development|PrintString "Picked up weapon"))
    (:then_1
      ;[0.15 0.15 0.15 0.5] Remove sphere collision
      (Components|DestroyComponent (Variables|Default|GetSphere)) ; Automatically invokes OnComponentEndOverlap so no need to unbind the event manually
    )
    (:then_2
      ;[0.15 0.15 0.15 0.5] Get weapon montages from player
      (bind _didsucceed (CallFunction|TryGettingWeaponAnimations))
      (if _didsucceed
        (Variables|Config|SetWeaponSockets (.SocketToAttachTo (Utilities|Struct|BreakS_WeaponAnimations (Variables|Animation|GetWeaponMontages))))
        (else
          (Development|PrintString "No Animation Montage found for the weapon tag" true true "(R=1.000000,G=0.050815,B=0.000000,A=1.000000)"))))))

(event Custom|HandleOnInteract
  (params (InteractionInitiator :type BP%20Character%20Base%20Object%20Reference))
  ;[0.15 0.15 0.15 0.5] Interact input/interface Handle
  (CallFunction|AddtoInventory InteractionInitiator))

(event Custom|HandleUnequipNotify
  (Transformation|AttachComponentToComponent (Variables|Default|GetSkeletalMesh) (Variables|/Script/Engine.Character|GetMesh (Variables|InventoryState|GetOwnerCharacter)) (.unequipped (.SocketToAttachTo (Utilities|Struct|BreakS_WeaponAnimations (Variables|Animation|GetWeaponMontages)))) "KeepRelative" "KeepRelative" "KeepRelative" true)
  (Default|ChangeIdleAnimation (Variables|InventoryState|GetOwnerCharacter))
  (Variables|InventoryState|SetEquipState "NewEnumerator4"))

(event Custom|HandleEquipNotify
  (Transformation|AttachComponentToComponent (Variables|Default|GetSkeletalMesh) (Variables|/Script/Engine.Character|GetMesh (Variables|InventoryState|GetOwnerCharacter)) (.equipped (.SocketToAttachTo (Utilities|Struct|BreakS_WeaponAnimations (Variables|Animation|GetWeaponMontages)))) "KeepRelative" "KeepRelative" "KeepRelative" true)
  (Default|ChangeIdleAnimation (Variables|InventoryState|GetOwnerCharacter) (Utilities|Array|Get(acopy) (.idle (Variables|Animation|GetWeaponMontages))))
  (Variables|InventoryState|SetEquipState "NewEnumerator2"))

(event Custom|InitiateAttack
  (Animation|Montage|PlayMontage (Variables|/Script/Engine.Character|GetMesh (Variables|InventoryState|GetOwnerCharacter)) (Utilities|Array|Get(acopy) (.attack (Variables|Animation|GetWeaponMontages))) 1.0 0.0 "None" false))

(event EventRecieveReloadNotify)

(event EventRecieveProjectileFiredNotify)

(event EventRecieveWeaponUnequippedNotify
  (CallFunction|HandleUnequipNotify))

(event EventRecieveWeaponEquippedNotify
  (CallFunction|HandleEquipNotify))

(event EventRecieveAttackedNotify)

(fn ConstructionScript)

(fn CanAttack
  (return true))

(fn TryGettingWeaponAnimations
  (bind _weapontypetag (Variables|Config|GetWeaponTypeTag))
  (bind _ownercharacter (Variables|InventoryState|GetOwnerCharacter))
  (bind _weaponinventory (Variables|/Game/Commons/Character/BP_CharacterBase.BP_CharacterBase_C|GetWeaponInventory _ownercharacter))
  (bind _weaponanimationmontagemap (Variables|/Game/Commons/Weapons/Blueprints/BPC_WeaponInventoryComponent.BPC_WeaponInventoryComponent_C|GetWeaponAnimationMontageMap _weaponinventory))
  (bind (_value _returnvalue) (Utilities|Map|Find _weaponanimationmontagemap _weapontypetag))
  (if _returnvalue
    (Variables|Animation|SetWeaponMontages _value)
    (return true)
    (else
      (return false))))

(fn AddtoInventory
  (params (Owner :type BP%20Character%20Base%20Object%20Reference))
  (Utilities|IsValid Owner
    (:Is%20Valid
      (bind _weaponinventory (Variables|/Game/Commons/Character/BP_CharacterBase.BP_CharacterBase_C|GetWeaponInventory Owner)
        (:then
          (bind _success (Default|TryAddWeapontoInventory _weaponinventory self))
          (if _success
            (CallFunction|OnWeaponPickedUp Owner)
            (else
              (Development|PrintString "Couldnt add to inventory" true true "(R=1.000000,G=0.070773,B=0.000000,A=1.000000)")))
          (return _success))
        (:else
          (Development|PrintString "Invalid Inventory to add weapon to" true true "(R=1.000000,G=0.072499,B=0.000000,A=1.000000)"))))
    (:Is%20Not%20Valid
      (Development|PrintString "Invalid Owner to add weapon to" true true "(R=1.000000,G=0.072499,B=0.000000,A=1.000000)"))))

(fn Interact
  (params (InteractionInsignator :type BP%20Character%20Base%20Object%20Reference%20%28by%20ref%29))
  (bind _success_ (CallFunction|AddtoInventory InteractionInsignator))
  (return _success_))

(fn ShouldInteract
  (return (not (Variables|InventoryState|GetHasBeenPickedUp))))