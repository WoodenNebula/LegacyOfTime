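; Magazine component that tracks a ranged weapon's loaded and reserve bullet counts and answers whether it can fire or reload.
; Init binds to the weapon's reload and switch state events and, for player-owned weapons, creates a bullet HUD widget.
; Firing decrements the magazine, and the reload notify refills it from the reserve, both broadcasting the new counts.
; Switch state changes hide the widget on unequip and show it when equipping.
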(event Custom|OnWeaponSwitchStateUpdated_Event
  (params (NewState :type E_WeaponEquipState%20Enum :default "NewEnumerator0"))
  (switch Utilities|FlowControl|Switch|SwitchonE_WeaponEquipState NewState
    (:NewEnumerator0
      (bind _w_bulletdisplay (Variables|HUD|GetW_BulletDisplay)
        (:then
          (Default|ToggleDisplayVisibility _w_bulletdisplay false))
        (:else)))
    (:NewEnumerator1
      (Variables|HUD|GetW_BulletDisplay
        (:then
          (Default|ToggleDisplayVisibility _w_bulletdisplay true))
        (:else)))))

(event Custom|OnWeaponReloadStateUpdated_Event
  (params (NewState :type E_WeaponReloadState%20Enum :default "NewEnumerator0") (MagBulletCount :type Integer) (RemainingBulletCount :type Integer))
  (switch Utilities|FlowControl|Switch|SwitchonE_WeaponReloadState NewState
    (:NewEnumerator1
      (bind (_inmag _remaining) (CallFunction|Reload))
      (Default|CallOnBulletCountUpdated _inmag _remaining))))

(event Custom|Init
  (params (WeaponAttachedTo :type BP%20Ranged%20Weapons%20Object%20Reference))
  (bind _output_get (Variables|Default|SetWeaponAttachedTo WeaponAttachedTo))
  (Utilities|IsValid _output_get
    (:Is%20Valid
      (Utilities|FlowControl|Sequence
        (:then_0
          (if (Default|IsPlayerCharacter? (Variables|/Game/Commons/Weapons/Blueprints/BP_Weapons.BP_Weapons_C|GetOwnerCharacter (Variables|Default|GetWeaponAttachedTo)))
            (bind _returnvalue (UserInterface|CreateWidget "/Game/Commons/Weapons/Widgets/WBP_Bullets.WBP_Bullets_C"))
            (bind _output_get_2 (Variables|HUD|SetW_BulletDisplay _returnvalue))
            (Utilities|FlowControl|DelayUntilNextTick)
            (Default|Init _output_get_2 (Variables|Default|GetBulletsCountInMag) (Variables|Default|GetRemainingBullets) (Variables|Default|GetMaxBulletsPerMag) self)))
        (:then_1
          (EventDispatchers|AssignOnWeaponReloadStateUpdated (Variables|Default|GetWeaponAttachedTo) (delegate Custom|OnWeaponReloadStateUpdated_Event))
          (EventDispatchers|AssignOnWeaponSwitchStateUpdated (Variables|Default|GetWeaponAttachedTo) (delegate Custom|OnWeaponSwitchStateUpdated_Event)))))))

(fn Reload
  (LocalVariables|SetReloadableAmount (- (Variables|Default|GetMaxBulletsPerMag) (Variables|Default|GetBulletsCountInMag)))
  (if (> (Variables|Default|GetRemainingBullets) (LocalVariables|GetReloadableAmount))
    (Variables|Default|SetRemainingBullets (- (Variables|Default|GetRemainingBullets) (LocalVariables|GetReloadableAmount)))
    (Variables|Default|SetBulletsCountInMag (Variables|Default|GetMaxBulletsPerMag))
    (else
      (Variables|Default|SetBulletsCountInMag (+ (Variables|Default|GetBulletsCountInMag) (Variables|Default|GetRemainingBullets)))
      (Variables|Default|SetRemainingBullets 0)))
  (return (Variables|Default|GetBulletsCountInMag) (Variables|Default|GetRemainingBullets)))

(fn CanReload
  (LocalVariables|SetDiff (- (Variables|Default|GetMaxBulletsPerMag) (Variables|Default|GetBulletsCountInMag)))
  (return (and (> (LocalVariables|GetDiff) 0) (> (Variables|Default|GetRemainingBullets) 0))))

(fn CanFire
  (return (> (Variables|Default|GetBulletsCountInMag) 0)))

(fn Fire
  (bind _result (Math|Integer|DecrementInt (Variables|Default|GetBulletsCountInMag))
    (:%20%20
      (Default|CallOnBulletCountUpdated _result (Variables|Default|GetRemainingBullets)))))