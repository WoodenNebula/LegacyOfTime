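; Ranged-weapon crosshair component that manages the crosshair widget and aim spread, broadcasting spread changes.
; Spread sums base, movement/jump and dynamic parts, capped at a maximum.
; A looping timer, active only while the crosshair shows, detects moving and falling, while a spawned helper actor's Timeline, rate-scaled by a recovery curve, drives dynamic spread recovery.
; GetTracePoint randomizes trace endpoints within a box scaled by spread and distance.
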(event EventBeginPlay
  (Utilities|FlowControl|Sequence
    (:then_0
      ;[0.15 0.15 0.15 0.5] Construct Widget if it doesnt exist
      (Variables|HUD|GetW_Crosshair
        (:then
          _)
        (:else
          (bind _returnvalue (UserInterface|CreateWidget "/Game/Commons/Weapons/Ranged/Crosshair/WBP_CrossHairs.WBP_CrossHairs_C"))
          (bind _output_get (Variables|HUD|SetW_Crosshair _returnvalue))
          (UserInterface|Viewport|AddtoViewport _output_get 0)))
      (Default|Init (Variables|HUD|GetW_Crosshair) self)
      (Widget|SetVisibility (Variables|HUD|GetW_Crosshair) "Collapsed"))
    (:then_1
      (bind _returnvalue_2 (Game|SpawnActorfromClass "/Game/Commons/Weapons/Ranged/Crosshair/Crosshair_Timeline.Crosshair_Timeline_C" (Math|Transform|MakeTransform "0, 0, 0" "0, 0, 0" "1.000000,1.000000,1.000000") "Undefined" "MultiplyWithRoot" (Components|GetOwner) 0))
      (Variables|Default|SetTimeline (Variables|/Game/Commons/Weapons/Ranged/Crosshair/Crosshair_Timeline.Crosshair_Timeline_C|GetTimeline _returnvalue_2))
      (Transformation|AttachActorToActor _returnvalue_2 (Components|GetOwner) "None" "KeepRelative" "KeepRelative" "KeepRelative" true)
      ;[0.15 0.15 0.15 0.5] Set a timer to update crosshair gap every .1 second according to the movement values while aiming
      (bind _returnvalue_3 (Utilities|Time|SetTimerbyFunctionName 0 "HandleMove&FallSpread" 0.1 true))
      (bind _output_get_2 (Variables|Default|SetUpdaterTimer _returnvalue_3))
      (Utilities|Time|PauseTimerbyHandle _output_get_2))))

(fn ShowCrossHairs
  (bind _updatertimer (Variables|Default|GetUpdaterTimer))
  (bind _w_crosshair (Variables|HUD|GetW_Crosshair)
    (:then
      (Widget|SetVisibility _w_crosshair "Visible")
      (if (and (Utilities|Time|IsValidTimerHandle _updatertimer) (Class|KismetSystemLibrary|IsTimerPausedHandle _updatertimer))
        (Utilities|Time|UnpauseTimerbyHandle (Variables|Default|GetUpdaterTimer))))
    (:else)))

(fn AddDynamicSpread
  (params (Spread :type Float%20%28double-precision%29) (RecoveryRate :type Float%20%28double-precision%29))
  (Variables|Spread|SetDynamicSpread (+ (Variables|Spread|GetDynamicSpread) (Math|Float|SelectFloat (- (Variables|Spread|GetMaxSpread) (Spread|GetSpreadValue)) Spread (> (+ (Spread|GetSpreadValue) Spread) (Variables|Spread|GetMaxSpread)))))
  (Components|Timeline|SetNewTime (Variables|Default|GetTimeline) (- 1.0 (Math|Float|SafeDivide (Variables|Spread|GetDynamicSpread) 1e+03)))
  (Audio|Components|Audio|Play (Variables|Default|GetTimeline))
  (Components|Timeline|SetPlayRate (Variables|Default|GetTimeline) (* (/ (Variables|Spread|GetDynamicSpread) 1e+03) (/ 1.0 (Math|Curves|GetFloatValue (Variables|Spread|GetSpreadRecoveryTimeCurve) (Variables|Spread|GetDynamicSpread))) RecoveryRate)))

(fn GetSpreadValue
  (return (Math|Float|Min(Float) (+ (Variables|Spread|GetDynamicSpread) (Variables|Spread|GetBaseSpread) (Variables|Spread|GetAdditionalSpread)) (Variables|Spread|GetMaxSpread))))

(fn UpdateSpreadTimeline
  (params (Direction :type ETimelineDirection%20Enum :default "Forward") (Value :type Float%20%28double-precision%29))
  (Variables|Spread|SetDynamicSpread (* 1e+03 Value))
  (Default|CallOnSpreadChanged (Spread|GetSpreadValue)))

(fn IsFalling
  (return (> (Math|Float|Absolute(Float) (.Z (Math|Vector|BreakVector (Transformation|GetVelocity (Variables|/Game/Commons/Weapons/Blueprints/BP_Weapons.BP_Weapons_C|GetOwnerCharacter (Variables|Default|GetAttachedWeapon)))))) 0.0)))

(fn IsMoving
  (return (> (Math|Vector|VectorLengthXY (Transformation|GetVelocity (Variables|/Game/Commons/Weapons/Blueprints/BP_Weapons.BP_Weapons_C|GetOwnerCharacter (Variables|Default|GetAttachedWeapon)))) 0.0)))

(fn HandleMove&FallSpread
  (Utilities|FlowControl|Sequence
    (:then_0
      (if (!= (Base|IsFalling) (Variables|Default|GetLastFalling))
        (bind _output_get (Variables|Default|SetLastFalling (not (Variables|Default|GetLastFalling))))
        (if _output_get
          (Variables|Spread|SetAdditionalSpread (+ (Variables|Spread|GetAdditionalSpread) (Variables|Spread|GetJumpSpread)))
          (Default|CallOnSpreadChanged (Spread|GetSpreadValue))
          (else
            (Variables|Spread|SetAdditionalSpread (- (Variables|Spread|GetAdditionalSpread) (Variables|Spread|GetJumpSpread)))
            (Spread|AddDynamicSpread (Variables|Spread|GetJumpSpread) (Variables|Spread|GetSpreadRecoveryRate))))))
    (:then_1
      (if (!= (Base|IsMoving) (Variables|Default|GetLastMoving))
        (bind _output_get_2 (Variables|Default|SetLastMoving (not (Variables|Default|GetLastMoving))))
        (if _output_get_2
          (Variables|Spread|SetAdditionalSpread (+ (Variables|Spread|GetAdditionalSpread) (Variables|Spread|GetMovementSpread)))
          (Default|CallOnSpreadChanged (Spread|GetSpreadValue))
          (else
            (Variables|Spread|SetAdditionalSpread (- (Variables|Spread|GetAdditionalSpread) (Variables|Spread|GetMovementSpread)))
            (Spread|AddDynamicSpread (Variables|Spread|GetMovementSpread) (Variables|Spread|GetSpreadRecoveryRate))))))))

(fn GetTracePoint
  (params (StartPoint :type Transform) (Distance :type Float%20%28double-precision%29) (SpreadScale :type Float%20%28double-precision%29))
  (bind (_location _rotation) (Math|Transform|BreakTransform StartPoint))
  (return _location (+ (* (Math|Vector|GetForwardVector _rotation) Distance) (Math|Random|RandomPointinBoundingBox _location (* (* (* (Spread|GetSpreadValue) SpreadScale) (/ Distance (Variables|Spread|GetCorrectionFactor))) "1.000000,1.000000,1.000000")))))

(fn SetDefaultSpread
  (params (Base :type Float%20%28double-precision%29) (Jump :type Float%20%28double-precision%29) (Movement :type Float%20%28double-precision%29) (Max :type Float%20%28double-precision%29))
  (Variables|Spread|SetMaxSpread Max)
  (LocalVariables|SetLocal_BaseSpread (Variables|Spread|GetBaseSpread))
  (Utilities|FlowControl|Sequence
    (:then_0
      (if (Variables|Default|GetLastFalling)
        (Variables|Spread|SetAdditionalSpread (- (Variables|Spread|GetAdditionalSpread) (Variables|Spread|GetJumpSpread)))
        (Variables|Spread|SetAdditionalSpread (+ (Variables|Spread|GetAdditionalSpread) Jump))))
    (:then_1
      (if (Variables|Default|GetLastMoving)
        (Variables|Spread|SetAdditionalSpread (- (Variables|Spread|GetAdditionalSpread) (Variables|Spread|GetMovementSpread)))
        (Variables|Spread|SetAdditionalSpread (+ (Variables|Spread|GetAdditionalSpread) Movement))))
    (:then_2
      (Variables|Spread|SetBaseSpread Base)
      (Variables|Spread|SetJumpSpread Jump)
      (Variables|Spread|SetMovementSpread Movement)
      (if (> (LocalVariables|GetLocal_BaseSpread) (Variables|Spread|GetBaseSpread))
        (Spread|AddDynamicSpread (- (LocalVariables|GetLocal_BaseSpread) (Variables|Spread|GetBaseSpread)) (Variables|Spread|GetSpreadRecoveryRate))
        (else
          (Default|CallOnSpreadChanged (Spread|GetSpreadValue)))))))

(fn HideCrossHairs
  (bind _w_crosshair (Variables|HUD|GetW_Crosshair)
    (:then
      (Widget|SetVisibility _w_crosshair "Collapsed")
      (Utilities|Time|PauseTimerbyHandle (Variables|Default|GetUpdaterTimer)))
    (:else)))

(fn TryResetSpread
  (Default|CallOnTryResetSpread))