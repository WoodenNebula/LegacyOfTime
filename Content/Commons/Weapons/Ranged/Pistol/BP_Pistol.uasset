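; Pistol weapon Blueprint that adjusts how the gun sits on its owning character when aiming starts and ends.
; It extends the parent's aim begin and end events, calling the inherited logic first.
; Aiming snaps the skeletal mesh to the Pistol_ADS socket on the owner's mesh, and ending the aim snaps it back to Pistol_Equipped.
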(event EventOnAimBegin
  (|CallParentFunction)
  (Transformation|AttachComponentToComponent (Variables|Default|GetSkeletalMesh) (Variables|/Script/Engine.Character|GetMesh (Variables|Default|GetOwnerCharacter)) "Pistol_ADS" "SnapToTarget" "SnapToTarget" "SnapToTarget" true))

(event EventOnAimEnd
  (|CallParentFunction)
  (Transformation|AttachComponentToComponent (Variables|Default|GetSkeletalMesh) (Variables|/Script/Engine.Character|GetMesh (Variables|Default|GetOwnerCharacter)) "Pistol_Equipped" "SnapToTarget" "SnapToTarget" "SnapToTarget" true))

(fn ConstructionScript)