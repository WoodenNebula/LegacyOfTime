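; Rifle weapon Blueprint that repositions its skeletal mesh on the owning character when aiming starts and stops.
; Both aim events call the parent implementation, then reattach the mesh to the character mesh, snapping to the Rifle_ADS socket for aiming and Rifle_Equipped otherwise.
; All other weapon behavior is left to the parent class, as the construction script is empty.
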(event EventOnAimBegin
  (|CallParentFunction)
  (Transformation|AttachComponentToComponent (Variables|Default|GetSkeletalMesh) (Variables|/Script/Engine.Character|GetMesh (Variables|Default|GetOwnerCharacter)) "Rifle_ADS" "SnapToTarget" "SnapToTarget" "SnapToTarget" true))

(event EventOnAimEnd
  (|CallParentFunction)
  (Transformation|AttachComponentToComponent (Variables|Default|GetSkeletalMesh) (Variables|/Script/Engine.Character|GetMesh (Variables|Default|GetOwnerCharacter)) "Rifle_Equipped" "SnapToTarget" "SnapToTarget" "SnapToTarget" true))

(fn ConstructionScript)