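; BP_Throwables is a throwable weapon Blueprint that tracks how many throwables are held against a maximum.
; TryAddThrowable increments Count while it is below MaxCount and returns whether the add succeeded.
; The construction script only calls the parent version, and no throwing logic appears in these graphs.
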(fn ConstructionScript
  (|CallParentFunction))

(fn TryAddThrowable
  (if (< (Variables|Default|GetCount) (Variables|Default|GetMaxCount))
    (Math|Integer|IncrementInt (Variables|Default|GetCount)
      (:%20%20
        (LocalVariables|SetSuccess true)))
    (else
      (LocalVariables|SetSuccess false)))
  (return (LocalVariables|GetSuccess)))