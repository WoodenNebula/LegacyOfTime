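; BP_AI_QuestGiver is a quest giver actor that shows an interaction prompt to a nearby player until its quest is accepted.
; Trigger sphere overlaps cache the player character, toggle the prompt widget and bind or unbind HandleInteract to that player's interaction event.
; While the player is inside, Tick turns the widget toward the camera.
; HandleInteract calls Interact, a stub returning false here, and ShouldInteract reports whether the quest remains unaccepted.
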(event OnComponentBeginOverlap(TriggerSphere)
  (params (OverlappedComponent :type Primitive%20Component%20Object%20Reference) (OtherActor :type Actor%20Object%20Reference) (OtherComp :type Primitive%20Component%20Object%20Reference) (OtherBodyIndex :type Integer) (bFromSweep :type Boolean) (SweepResult :type Hit%20Result%20Structure%20%28by%20ref%29))
  ;[0.15 0.15 0.15 0.5] Widget Visibility on collision
  (if (not (Variables|Default|GetbHasAcceptedQuest?))
    (Variables|Default|GetInteractingPlayer
      (:then
        _)
      (:else
        (bind _asbp_player_character_base (Utilities|Casting|CastToBP_PlayerCharacterBase OtherActor))
        (bind _output_get (Variables|Default|SetInteractingPlayer _asbp_player_character_base))))
    (Variables|Default|SetbPlayerIsInArea true)
    (Rendering|SetVisibility (Variables|Default|GetInteract%20Widget) true false)
    (EventDispatchers|BindEventtoOnInteractionTriggered _output_get (delegate Custom|HandleInteract))))

(event OnComponentEndOverlap(TriggerSphere)
  (params (OverlappedComponent :type Primitive%20Component%20Object%20Reference) (OtherActor :type Actor%20Object%20Reference) (OtherComp :type Primitive%20Component%20Object%20Reference) (OtherBodyIndex :type Integer))
  ;[0.15 0.15 0.15 0.5] Widget Visibility on collision
  (Variables|Default|GetInteractingPlayer
    (:then
      _)
    (:else
      (bind _asbp_player_character_base (Utilities|Casting|CastToBP_PlayerCharacterBase OtherActor))
      (bind _output_get (Variables|Default|SetInteractingPlayer _asbp_player_character_base))))
  (Variables|Default|SetbPlayerIsInArea false)
  (Rendering|SetVisibility (Variables|Default|GetInteract%20Widget) false false)
  (EventDispatchers|UnbindEventfromOnInteractionTriggered _output_get (delegate Custom|HandleInteract)))

(event Custom|HandleInteract
  (params (InteractionInitiator :type BP%20Character%20Base%20Object%20Reference))
  (CallFunction|Interact InteractionInitiator))

(event EventTick
  (params (DeltaSeconds :type Float%20%28single-precision%29))
  (if (not (Variables|Default|GetbHasAcceptedQuest?))
    ;[0.15 0.15 0.15 0.5] Widget Rotation according to player camera
    (if (Variables|Default|GetbPlayerIsInArea)
      (Transformation|SetWorldRotation (Variables|Default|GetInteract%20Widget) (Math|Rotator|FindLookatRotation (Transformation|GetWorldLocation (Variables|Default|GetInteract%20Widget)) (Transformation|GetWorldLocation (Variables|/Script/Engine.PlayerCameraManager|GetTransformComponent (Game|GetPlayerCameraManager 0)))) false false))))

(fn ConstructionScript)

(fn Interact
  (params (InteractionInsignator :type BP%20Character%20Base%20Object%20Reference%20%28by%20ref%29))
  (return false))

(fn ShouldInteract
  (return (not (Variables|Default|GetbHasAcceptedQuest?))))