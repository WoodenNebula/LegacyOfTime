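; BP_DarkEve is an Eve character variant that acts as a scripted, rifle-armed attacker against the player.
; On BeginPlay it spawns a BP_Rifle and adds it to its own inventory.
; When an actor tagged Player overlaps its Box, it selects the primary weapon, rotates toward that actor, then starts aiming and attacking after short delays.
; It drives inherited input handlers directly, with no stop logic in this graph.
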(event OnComponentBeginOverlap(Box)
  (params (OverlappedComponent :type Primitive%20Component%20Object%20Reference) (OtherActor :type Actor%20Object%20Reference) (OtherComp :type Primitive%20Component%20Object%20Reference) (OtherBodyIndex :type Integer) (bFromSweep :type Boolean) (SweepResult :type Hit%20Result%20Structure%20%28by%20ref%29))
  (if (Actor|ActorHasTag OtherActor "Player")
    (CallFunction|HandlePrimaryWeaponSelectInput)
    (Transformation|AddActorLocalRotation (Math|Rotator|FindRelativeLookatRotation (Transformation|GetActorTransform) (Transformation|GetActorLocation OtherActor)) false false)
    (Utilities|FlowControl|Delay 1.0)
    (CallFunction|HandleAimStartInput)
    (Utilities|FlowControl|Delay 1.0)
    (CallFunction|HandleAttackStartInput)))

(event EventBeginPlay
  (|CallParentFunction)
  (bind _returnvalue (Game|SpawnActorfromClass "/Game/Commons/Weapons/Ranged/Rifle/BP_Rifle.BP_Rifle_C" (Transformation|GetActorTransform) "AlwaysSpawn" "MultiplyWithRoot" self 0))
  (Default|AddtoInventory _returnvalue self))

(fn ConstructionScript)