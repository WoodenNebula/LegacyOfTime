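; Parent building Blueprint that applies configurable wall, wood trim, footer and roof looks to its modular mesh pieces.
; The construction script creates dynamic material instances for outer walls, exterior wood and footer, tinting each through its AlbedoColor parameter.
; It assigns them by material slot name to static mesh children of Walls, with the footer material also covering Footer children.
; The RoofTypes selection picks one of three roof materials for the Roof slot on Walls children.
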(fn ConstructionScript
  ;[1 1 1] Color Tweaks
  ;;[1 1 1] Set Exterior Wall Colors
  (bind _returnvalue (Rendering|Material|CreateDynamicMaterialInstance "/Game/SurabGame/PostDistrict/Materials/Structure/Outer/MI_WoodenWall.MI_WoodenWall" "None" "None" :!class /Script/Engine.KismetMaterialLibrary))
  (bind _output_get (Variables|Default|SetExternalWallInst _returnvalue))
  (Rendering|Material|SetVectorParameterValue _output_get "AlbedoColor" (Variables|Walls|GetOuterWallColor) :!class /Script/Engine.MaterialInstanceDynamic)
  (for _array_element (Components|GetChildrenComponents (Variables|Default|GetWalls) false)
    (bind _asstatic_mesh_component (Utilities|Casting|CastToStaticMeshComponent _array_element))
    (Rendering|Material|SetMaterialbyName _asstatic_mesh_component "OuterWoodPanels" (Variables|Default|GetExternalWallInst)))
  ;;[1 1 1] Set Wood Color
  (bind _returnvalue_2 (Rendering|Material|CreateDynamicMaterialInstance "/Game/SurabGame/PostDistrict/Materials/Structure/Outer/MI_OuterWood.MI_OuterWood" "None" "None" :!class /Script/Engine.KismetMaterialLibrary))
  (bind _output_get_2 (Variables|Default|SetExternalWoodInst _returnvalue_2))
  (Rendering|Material|SetVectorParameterValue _output_get_2 "AlbedoColor" (Variables|Walls|GetExternalWoodColor) :!class /Script/Engine.MaterialInstanceDynamic)
  (for _array_element_2 (Components|GetChildrenComponents (Variables|Default|GetWalls) false)
    (bind _asstatic_mesh_component_2 (Utilities|Casting|CastToStaticMeshComponent _array_element_2))
    (Rendering|Material|SetMaterialbyName _asstatic_mesh_component_2 "LightWoodTrim" (Variables|Default|GetExternalWoodInst)))
  ;;[1 1 1] Set Footer Color
  (bind _returnvalue_3 (Rendering|Material|CreateDynamicMaterialInstance "/Game/SurabGame/PostDistrict/Materials/Structure/Outer/MI_FooterWall.MI_FooterWall" "None" "None" :!class /Script/Engine.KismetMaterialLibrary))
  (bind _output_get_3 (Variables|Default|SetFooterInst _returnvalue_3))
  (Rendering|Material|SetVectorParameterValue _output_get_3 "AlbedoColor" (Variables|Walls|GetFooterColor) :!class /Script/Engine.MaterialInstanceDynamic)
  (for _array_element_3 (Components|GetChildrenComponents (Variables|Default|GetFooter) false)
    (bind _asstatic_mesh_component_3 (Utilities|Casting|CastToStaticMeshComponent _array_element_3))
    (Rendering|Material|SetMaterialbyName _asstatic_mesh_component_3 "Footer" (Variables|Default|GetFooterInst)))
  (for _array_element_4 (Components|GetChildrenComponents (Variables|Default|GetWalls) false)
    (bind _asstatic_mesh_component_4 (Utilities|Casting|CastToStaticMeshComponent _array_element_4))
    (Rendering|Material|SetMaterialbyName _asstatic_mesh_component_4 "Footer" (Variables|Default|GetFooterInst)))
  ;[1 1 1] Set Roof Type
  (for _array_element_5 (Components|GetChildrenComponents (Variables|Default|GetWalls) false)
    (bind _asstatic_mesh_component_5 (Utilities|Casting|CastToStaticMeshComponent _array_element_5))
    (Rendering|Material|SetMaterialbyName _asstatic_mesh_component_5 "Roof" (Utilities|Select :Index (Variables|Structure|GetRoofTypes) :NewEnumerator0 "/Game/SurabGame/PostDistrict/Materials/Structure/Outer/MI_TileRoof_Hexa.MI_TileRoof_Hexa" :NewEnumerator2 "/Game/SurabGame/PostDistrict/Materials/Structure/Outer/MI_MetalRoof.MI_MetalRoof" :NewEnumerator3 "/Game/SurabGame/PostDistrict/Materials/Structure/Outer/MI_TileRoof_Red.MI_TileRoof_Red"))))